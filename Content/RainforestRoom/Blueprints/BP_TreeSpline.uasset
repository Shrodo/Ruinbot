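; Spline actor for the rainforest room that builds a tapered mesh along a spline, likely a tree trunk or branch.
; Its construction script adds one spline mesh component per segment, using the exposed mesh, material and forward axis, with positions and tangents from the spline points.
; Cross-section scale lerps from start to end radius by distance along the spline, giving a continuous taper across segments.
; The event graph is unused.
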(fn `UserConstructionScript`
  (bind _spline1 (`self.Spline1`))
  (bind _returnvalue (`SplineComponent.GetNumberOfSplinePoints` _spline1))
  (bind _returnvalue_2 (/ (`self.EndRadius`) 100.0))
  (bind _returnvalue_3 (/ (`self.StartRadius`) 100.0))
  (bind _returnvalue_4 (`SplineComponent.GetDistanceAlongSplineAtSplinePoint` _spline1 (- _returnvalue 1)))
  (for _index (range (+ (- _returnvalue 2) 1))
    (bind _returnvalue_5 (`AddComponent|NODE_AddSplineMeshComponent-1`))
    (`StaticMeshComponent.SetStaticMesh` _returnvalue_5 (`self.StaticMesh`))
    (`PrimitiveComponent.SetMaterial` _returnvalue_5 0 (`self.Material`))
    (`SplineMeshComponent.SetForwardAxis` _returnvalue_5 (`self.ForwardAxis`) true)
    (`SceneComponent.K2_AttachToComponent` _returnvalue_5 _spline1 "None" "KeepRelative" "KeepRelative" "KeepRelative" true)
    (bind _returnvalue_6 (+ _index 1))
    (`SplineMeshComponent.SetStartAndEnd` _returnvalue_5 (`SplineComponent.GetLocationAtSplinePoint` _spline1 _index "Local") (`SplineComponent.GetTangentAtSplinePoint` _spline1 _index "Local") (`SplineComponent.GetLocationAtSplinePoint` _spline1 _returnvalue_6 "Local") (`SplineComponent.GetTangentAtSplinePoint` _spline1 _returnvalue_6 "Local") true)
    (bind _returnvalue_7 (`KismetMathLibrary.Lerp` _returnvalue_3 _returnvalue_2 (/ (`SplineComponent.GetDistanceAlongSplineAtSplinePoint` _spline1 _index) _returnvalue_4)))
    (`SplineMeshComponent.SetStartScale` _returnvalue_5 (`KismetMathLibrary.MakeVector2D` _returnvalue_7 _returnvalue_7) true)
    (bind _returnvalue_8 (`KismetMathLibrary.Lerp` _returnvalue_3 _returnvalue_2 (/ (`SplineComponent.GetDistanceAlongSplineAtSplinePoint` _spline1 _returnvalue_6) _returnvalue_4)))
    (`SplineMeshComponent.SetEndScale` _returnvalue_5 (`KismetMathLibrary.MakeVector2D` _returnvalue_8 _returnvalue_8) true)))