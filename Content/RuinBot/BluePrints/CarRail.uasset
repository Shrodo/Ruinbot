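; CarRail is a spline-based rail actor that snaps a hand-placed spline to a modular grid.
; The construction script rounds each point's position and tangent direction to fixed steps, gives tangents a uniform TangentLength, and adds a spline mesh per segment.
; It also caches the snapped values in RailPointsRounded and RailTangentsRounded.
; BeginPlay rebuilds RailSpline from those arrays, so the runtime spline follows the snapped meshes.
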(event `self.ReceiveBeginPlay`
  (bind _railspline (`self.RailSpline`))
  (`SplineComponent.ClearSplinePoints` _railspline false)
  (for (_array_element _array_index) (`self.RailPointsRounded`)
    (`SplineComponent.AddSplinePointAtIndex` _railspline _array_element _array_index "Local" false)
    (`SplineComponent.SetTangentAtSplinePoint` _railspline _array_index (`|GetArrayItem` (`self.RailTangentsRounded`) _array_index) "Local" true)))

(fn `UserConstructionScript`
  (bind _railspline (`self.RailSpline`))
  (bind _returnvalue (- (`SplineComponent.GetNumberOfSplinePoints` _railspline) 1))
  (for _index (range (+ _returnvalue 1))
    (if (not (== _index _returnvalue))
      (bind _returnvalue_2 (`AddComponent|NODE_AddSplineMeshComponent-1`))
      (bind (_location _tangent) (`SplineComponent.GetLocationAndTangentAtSplinePoint` _railspline _index "Local"))
      (bind _returnvalue_3 (`KismetMathLibrary.MakeVector` (* (`KismetMathLibrary.Conv_IntToDouble` (`KismetMathLibrary.Round` (/ (.x _location) 250.0))) 250.0) (* (`KismetMathLibrary.Conv_IntToDouble` (`KismetMathLibrary.Round` (/ (.y _location) 250.0))) 250.0) (* (`KismetMathLibrary.Conv_IntToDouble` (`KismetMathLibrary.Round` (/ (.z _location) 100.0))) 100.0)))
      (bind _returnvalue_4 (* (`KismetMathLibrary.GetForwardVector` (`KismetMathLibrary.MakeRotator` (* (`KismetMathLibrary.Round` (/ (.roll (`KismetMathLibrary.FindLookAtRotation` (`KismetMathLibrary.MakeVector` 0.0) _tangent)) 30.0)) 30.0) (* (`KismetMathLibrary.Round` (/ (.pitch (`KismetMathLibrary.FindLookAtRotation` (`KismetMathLibrary.MakeVector` 0.0) _tangent)) 30.0)) 30.0) (* (`KismetMathLibrary.Round` (/ (.yaw (`KismetMathLibrary.FindLookAtRotation` (`KismetMathLibrary.MakeVector` 0.0) _tangent)) 45.0)) 45.0))) (`self.TangentLength`)))
      (bind (_location_2 _tangent_2) (`SplineComponent.GetLocationAndTangentAtSplinePoint` _railspline (+ _index 1) "Local"))
      (`SplineMeshComponent.SetStartAndEnd` _returnvalue_2 _returnvalue_3 _returnvalue_4 (`KismetMathLibrary.MakeVector` (* (`KismetMathLibrary.Conv_IntToDouble` (`KismetMathLibrary.Round` (/ (.x _location_2) 250.0))) 250.0) (* (`KismetMathLibrary.Conv_IntToDouble` (`KismetMathLibrary.Round` (/ (.y _location_2) 250.0))) 250.0) (* (`KismetMathLibrary.Conv_IntToDouble` (`KismetMathLibrary.Round` (/ (.z _location_2) 100.0))) 100.0)) (* (`KismetMathLibrary.GetForwardVector` (`KismetMathLibrary.MakeRotator` (* (`KismetMathLibrary.Round` (/ (.roll (`KismetMathLibrary.FindLookAtRotation` (`KismetMathLibrary.MakeVector` 0.0) _tangent_2)) 30.0)) 30.0) (* (`KismetMathLibrary.Round` (/ (.pitch (`KismetMathLibrary.FindLookAtRotation` (`KismetMathLibrary.MakeVector` 0.0) _tangent_2)) 30.0)) 30.0) (* (`KismetMathLibrary.Round` (/ (.yaw (`KismetMathLibrary.FindLookAtRotation` (`KismetMathLibrary.MakeVector` 0.0) _tangent_2)) 45.0)) 45.0))) (`self.TangentLength`)) true))
    (`KismetArrayLibrary.Array_Set` (`self.RailPointsRounded`) _index _returnvalue_3 true)
    (`KismetArrayLibrary.Array_Set` (`self.RailTangentsRounded`) _index _returnvalue_4 true)))