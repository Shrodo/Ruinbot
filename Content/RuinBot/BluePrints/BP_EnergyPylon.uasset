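; BP_EnergyPylon is a chargeable pylon that drives an Actor Sequence on a target actor, picked by component index.
; BeginPlay caches the sequence player and leaves it primed and paused.
; ChargeAction alternates a timeline forward and backward, whose signed speed sets playback rate and direction.
; Hold-charge events loop the sequence while a second timeline ramps its speed, reversing on release and pausing when finished at zero.
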(event `self.ReceiveBeginPlay`
  (bind _target_actor (`self.Target Actor`)
    (:`then`
      (bind _sequenceplayer (`ActorSequenceComponent.SequencePlayer` (`|GetArrayItem` (`self.K2_GetComponentsByClass` _target_actor "/Script/ActorSequence.ActorSequenceComponent") (`self.SeqID`))))
      (`MovieSceneSequencePlayer.SetPlayRate` _sequenceplayer 0.0)
      (bind _output_get (set `self.SeqPlayer` _sequenceplayer))
      (`MovieSceneSequencePlayer.Play` _output_get)
      (`MovieSceneSequencePlayer.Pause` _output_get))
    (:`else`)))

(event `ChargeAction`
  (`|ExecutionSequence`
    (:`then_0`
      (bind (_direction _seqspeed) (`Timeline|Timeline_1` :`NewTime` 0.5 :!via `SetNewTime` :!label _label)
        (:`Update`
          (bind _seqplayer (`self.SeqPlayer`)
            (:`then`
              (`MovieSceneSequencePlayer.SetPlayRate` _seqplayer (`KismetMathLibrary.Abs` _seqspeed))
              (if (< _seqspeed 0.0)
                (`MovieSceneSequencePlayer.PlayReverse` _seqplayer)
                (else
                  (`MovieSceneSequencePlayer.Play` _seqplayer))))
            (:`else`)))))
    (:`then_1`
      (`/Engine/EditorBlueprintResources/StandardMacros.FlipFlop`
        (:`A`
          (goto _label))
        (:`B`
          (goto _label :!via `Reverse`))))))

(event `HoldChargeStart`
  (bind _seqplayer (`self.SeqPlayer`))
  (`MovieSceneSequencePlayer.PlayLooping` _seqplayer -1)
  (bind (_direction _seqspeed) (`Timeline|Timeline_0` :!label _label_2)
    (:`Update`
      (`MovieSceneSequencePlayer.SetPlayRate` _seqplayer _seqspeed))
    (:`Finished`
      (if (== _seqspeed 0.0)
        (`MovieSceneSequencePlayer.Pause` _seqplayer)))))

(event `HoldChargeEnd`
  (goto _label_2 :!via `Reverse`))

(fn `UserConstructionScript`)