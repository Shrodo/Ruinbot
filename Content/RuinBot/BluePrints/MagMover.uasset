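; MagMover is a temporarily possessed pawn that plots a grid path for RuinBot's magnet target.
; Camera-relative input snaps to world-axis steps on a cooldown, box-tracing a copied collision mesh to block obstructed moves.
; Each step records its location and spawns a trail actor, while backtracking or AltToggle removes the last.
; Jump sends the path to the target's MagneticObject and AimedGadget clears the trail, both returning possession to MasterPawn before self-destructing.
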(event `self.ReceiveBeginPlay`
  (bind _camboom (`self.CamBoom`))
  (`SceneComponent.K2_SetWorldRotation` (`self.MagCam`) (struct :`Pitch` -0.5) false false)
  (`SceneComponent.K2_SetWorldRotation` _camboom (`KismetMathLibrary.MakeRotator` 0.0 -30.0 (`self.CamRotZ`)) false false)
  (set `SpringArmComponent.TargetArmLength` 15000.0 _camboom)
  ;[1 1 1] Set collision mesh from spawn input variables
  (bind _collisionmesh (`self.CollisionMesh`)
    (:`then`
      (bind _returnvalue (`AddComponent|NODE_AddStaticMeshComponent-0` :`RelativeTransform` (`KismetMathLibrary.ConvertTransformToRelative` (`self.GetTransform`) (`self.CollisionTF`))))
      (`StaticMeshComponent.SetStaticMesh` _returnvalue _collisionmesh)
      (bind _output_get (set `self.Collision` _returnvalue))
      (bind _returnvalue_2 (`KismetMaterialLibrary.CreateDynamicMaterialInstance` "/Game/RuinBot/TexMat/M_MagMoverCollision.M_MagMoverCollision"))
      (for (_ _array_index) (`MeshComponent.GetMaterials` _returnvalue)
        (`PrimitiveComponent.SetMaterial` _output_get _array_index _returnvalue_2)))
    (:`else`)))

(event `InputAction|AltToggle`
  (params (Key :type "Key Structure"))
  (bind _magmovelocations (`self.MagMoveLocations`))
  (bind _returnvalue (`KismetArrayLibrary.Array_Length` _magmovelocations))
  (bind _returnvalue_2 (- _returnvalue 1))
  (:`Pressed`
    (if (> (`KismetArrayLibrary.Array_Length` _magmovelocations) 0)
      (`KismetArrayLibrary.Array_Remove` _magmovelocations _returnvalue_2 :!label _label)
      (`self.K2_DestroyActor` (`|GetArrayItem` (`self.MagMoveActors`) _returnvalue))
      (set `self.NewLoc` (`self.LastLoc`))
      (set `self.LastLoc` (`|GetArrayItem` _magmovelocations _returnvalue_2))
      (`self.K2_SetActorLocation` (`self.NewLoc`))
      (set `self.MoveCool` false)
      (`KismetSystemLibrary.K2_SetTimer` null "MoveCooldown" 0.2))))

(event `InputAxis|MoveForward`
  (params (AxisValue :type "Float (single-precision)"))
  (bind _returnvalue (`self.K2_GetActorLocation`))
  (bind _gridsize (`self.GridSize`))
  (bind _magmovelocations (`self.MagMoveLocations`))
  (bind (_origin _boxextent) (`KismetSystemLibrary.GetComponentBounds` (`self.Collision`)))
  (bind _returnvalue_2 (* _gridsize -1.0))
  (bind _returnvalue_3 (`KismetMathLibrary.MakeRotator` 0.0 0.0 (.yaw (`SceneComponent.K2_GetComponentRotation` (`self.MagCam`)))))
  (bind _returnvalue_4 (`KismetMathLibrary.MakeVector` (.x (`self.NewLoc`)) (.y (`self.NewLoc`)) (.z _origin)))
  (bind _x (.x (+ (* (`KismetMathLibrary.GetForwardVector` _returnvalue_3) AxisValue) (* (`KismetMathLibrary.GetRightVector` _returnvalue_3) (stale `InputAxis|MoveRight` AxisValue)))))
  (bind _y (.y (+ (* (`KismetMathLibrary.GetForwardVector` _returnvalue_3) AxisValue) (* (`KismetMathLibrary.GetRightVector` _returnvalue_3) (stale `InputAxis|MoveRight` AxisValue)))))
  (bind _returnvalue_5 (`KismetMathLibrary.Abs` _y))
  (bind _returnvalue_6 (`KismetMathLibrary.Abs` _x))
  (if (and (`self.MoveCool`) (or (> _returnvalue_5 0.5) (> _returnvalue_6 0.5))) :!label _label_2
    (if (>= _returnvalue_6 _returnvalue_5)
      (if (>= _x 0.0)
        (set `self.DirectionMove` 0)
        (else
          (set `self.DirectionMove` 1)))
      (elif (>= _y 0.0)
        (set `self.DirectionMove` 2)
        (else
          (set `self.DirectionMove` 3))))
    (bind _output_get (set `self.NewLoc` (+ _returnvalue (select `int` (`self.DirectionMove`) :`0` (`KismetMathLibrary.MakeVector` _gridsize) :`1` (`KismetMathLibrary.MakeVector` _returnvalue_2) :`2` (`KismetMathLibrary.MakeVector` 0.0 _gridsize) :`3` (`KismetMathLibrary.MakeVector` 0.0 _returnvalue_2)))))
    (if (`KismetArrayLibrary.Array_Contains` _magmovelocations _output_get)
      (if (== _output_get (`self.LastLoc`))
        (goto _label))
      (else
        (bind (_outhit _returnvalue_7) (`KismetSystemLibrary.BoxTraceSingle` (`KismetMathLibrary.VLerp` _origin _returnvalue_4 0.3) _returnvalue_4 (* _boxextent (0.8 0.8 0.8)) (struct) "TraceTypeQuery1" false (`|MakeArray` (`self.MasterPawn`) (`self.MagTarget`) :!type "Actor Object Reference")))
        (`KismetSystemLibrary.PrintString` (`KismetSystemLibrary.GetDisplayName` (`.HitActor` (`GameplayStatics.BreakHitResult` _outhit))))
        (if (not _returnvalue_7)
          (bind _output_get_2 (set `self.LastLoc` _returnvalue))
          (`self.K2_SetActorLocation` (`self.NewLoc`))
          (bind _returnvalue_8 (`KismetArrayLibrary.Array_AddUnique` _magmovelocations _output_get_2))
          (bind _returnvalue_9 (`|SpawnActorFromClass` "/Game/RuinBot/BluePrints/MagMoverTrail.MagMoverTrail_C" (`KismetMathLibrary.Conv_VectorToTransform` _output_get_2) "AlwaysSpawn" "OverrideRootScale" self null))
          (`PrimitiveComponent.CreateDynamicMaterialInstance` (`/Game/RuinBot/BluePrints/MagMoverTrail.Cube` _returnvalue_9) 0 null "None")
          (`KismetArrayLibrary.Array_Set` (`self.MagMoveActors`) _returnvalue_8 _returnvalue_9 true)
          (set `self.MoveCool` false)
          (`KismetSystemLibrary.K2_SetTimer` null "MoveCooldown" 0.2))))))

(event `InputAxis|MoveRight`
  (params (AxisValue :type "Float (single-precision)"))
  (goto _label_2))

(event `MoveCooldown`
  (set `self.MoveCool` true))

(event `SetMasterPawn`
  (params (Pawn :type "Pawn Object Reference"))
  (bind _output_get (set `self.MasterPawn` Pawn))
  (bind _asruin_bot_test_char (cast `/Game/RuinBot/Character/RuinBotTestChar` _output_get))
  (set `self.MagTarget` (`/Game/RuinBot/Character/RuinBotTestChar.MagnetTargetActor` _asruin_bot_test_char)))

(event `InputAction|AimedGadget`
  (params (Key :type "Key Structure"))
  (bind _masterpawn (`self.MasterPawn`))
  (:`Pressed`
    (for _array_element (`self.MagMoveActors`)
      (`/Engine/EditorBlueprintResources/StandardMacros.IsValid` _array_element
        (:`Is Valid`
          (`self.K2_DestroyActor` _array_element))))
    (`Controller.Possess` (`GameplayStatics.GetPlayerController` 0) _masterpawn :!label _label_3)
    (bind _asruin_bot_test_char (cast `/Game/RuinBot/Character/RuinBotTestChar` _masterpawn))
    (`/Game/RuinBot/Character/RuinBotTestChar.MagMoveOff` _asruin_bot_test_char self)
    (`MaterialInstanceDynamic.SetVectorParameterValue` (stale `self.ReceiveBeginPlay` _returnvalue_2) "Color" (struct :`R` 1.0 :`G` 1.0 :`B` 1.0 :`A` 1.0))
    (`SceneComponent.SetVisibility` (`self.Cube`) false false)
    (`KismetSystemLibrary.Delay` 0.5)
    (`/Engine/EditorBlueprintResources/StandardMacros.IsValid` self
      (:`Is Valid`
        (`self.K2_DestroyActor`)))))

(event `InputAction|Jump`
  (params (Key :type "Key Structure"))
  (bind _returnvalue (`self.K2_GetActorLocation`))
  (bind _magmoveactors (`self.MagMoveActors`))
  (:`Pressed`
    (bind _returnvalue_2 (`KismetArrayLibrary.Array_AddUnique` (`self.MagMoveLocations`) _returnvalue))
    (bind _returnvalue_3 (`|SpawnActorFromClass` "/Game/RuinBot/BluePrints/MagMoverTrail.MagMoverTrail_C" (`KismetMathLibrary.Conv_VectorToTransform` _returnvalue) "AlwaysSpawn" "OverrideRootScale" self null))
    (`KismetArrayLibrary.Array_Set` _magmoveactors _returnvalue_2 _returnvalue_3 true)
    (`/Game/RuinBot/BluePrints/MagneticObject.MagnetMove` (`self.GetComponentByClass` (`self.MagTarget`) "/Game/RuinBot/BluePrints/MagneticObject.MagneticObject_C") (`self.MagMoveLocations`) _magmoveactors)
    (goto _label_3)))

(fn `UserConstructionScript`)