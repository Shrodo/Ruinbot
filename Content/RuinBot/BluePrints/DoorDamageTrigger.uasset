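; DoorDamageTrigger is a Blueprint attached to a BP_Door that opens it when damage of a type it is vulnerable to lands.
; On BeginPlay it caches the owning door and looks for a LocationMarker among the door's attached actors.
; DamageTaken checks the damage type against VulnerableTo, then opens the door and, if a marker was found, starts that marker's door-open timer.
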(event `self.ReceiveBeginPlay`
  (bind _asbp_door (cast `/Game/RuinBot/BluePrints/BP_Door` (`self.GetOwner`)))
  (set `self.Door` _asbp_door)
  (for _array_element (`Actor.GetAttachedActors` _asbp_door)
    (bind _aslocation_marker (cast `/Game/RuinBot/BluePrints/LocationMarker` _array_element))
    (set `self.LocationMarker` _aslocation_marker)))

(event `DamageTaken`
  (params (DamageType :type "/Game/RuinBot/BluePrints/DamageTypes Enum" :default "NewEnumerator0"))
  (if (`KismetArrayLibrary.Array_Contains` (`self.VulnerableTo`) DamageType)
    (`/Game/RuinBot/BluePrints/BP_Door.DoorOpen` (`self.Door`))
    (bind _locationmarker (`self.LocationMarker`)
      (:`then`
        (`/Game/RuinBot/BluePrints/LocationMarker.SetDoorOpenTimer` _locationmarker))
      (:`else`))))