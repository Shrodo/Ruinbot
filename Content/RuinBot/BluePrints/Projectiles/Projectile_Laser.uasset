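; Laser projectile that damages what it overlaps or is told it hit, ignoring its instigator.
; A hit plays a pitch-randomized sound, spawns an impact actor, passes death force direction to AI, applies laser damage and notifies door damage triggers.
; Non-piercing lasers then destroy themselves.
; Homing is manual: setting a target starts a looping timer that, when Homing is enabled, snaps rotation toward it and resets forward velocity.
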(event `self.Collision.OnComponentBeginOverlap`
  (params (OverlappedComponent :type "PrimitiveComponent Object Reference") (OtherActor :type "Actor Object Reference") (OtherComp :type "PrimitiveComponent Object Reference") (OtherBodyIndex :type Integer) (bFromSweep :type Boolean) (SweepResult :type "HitResult Structure (by ref)"))
  (`self.Hit/Over` OtherActor (`SceneComponent.GetForwardVector` (`self.SM_LaserMesh`)) SweepResult_ImpactPoint))

(event `SetHomingTarget`
  (params (HTarget :type "SceneComponent Object Reference"))
  (set `self.HomingTarget` HTarget)
  (`KismetSystemLibrary.K2_SetTimerDelegate` (delegate `ReAim`) 0.1 true))

(event `Hit/Over`
  (params (Other :type "Actor Object Reference") (HitNormal :type "Vector Structure") (HitLoc :type "Vector Structure"))
  (`/Engine/EditorBlueprintResources/StandardMacros.IsValid` Other
    (:`Is Valid`
      (set `self.HitActor` Other)
      (if (!= Other (`self.GetInstigator`))
        (bind _asai_entity (cast `/Game/RuinBot/AI/AI_Entity` Other)
          (:`then`
            (set `/Game/RuinBot/AI/AI_Entity.DeathForceVec` HitNormal _asai_entity)
            (bind _asnpc_char (cast `/Game/RuinBot/AI/NPC_Char` Other)
              (:`then`
                (set `/Game/RuinBot/AI/NPC_Char.DeathForceVec` HitNormal _asnpc_char))
              (:`CastFailed`
                _)))
          (:`CastFailed`
            _))
        (`GameplayStatics.PlaySoundAtLocation` (`self.ImpactSound`) HitLoc (struct) 1.0 (`KismetMathLibrary.RandomFloatInRange` 0.7 1.3) 0.0 null null null)
        (`|SpawnActorFromClass` (`self.ImpactBP`) (`KismetMathLibrary.MakeTransform` (.location (`SceneComponent.K2_GetComponentToWorld` (`self.SM_LaserMesh`))) (.rotation (`SceneComponent.K2_GetComponentToWorld` (`self.SM_LaserMesh`)))) "Undefined" "OverrideRootScale" null null)
        (bind _hitactor (`self.HitActor`)
          (:`then`
            (`GameplayStatics.ApplyDamage` _hitactor (`self.Damage`) (`self.GetInstigatorController`) self "/Game/RuinBot/BluePrints/BasicLaserDamage.BasicLaserDamage_C")
            (bind _returnvalue (`self.GetComponentByClass` _hitactor "/Game/RuinBot/BluePrints/DoorDamageTrigger.DoorDamageTrigger_C"))
            (`/Engine/EditorBlueprintResources/StandardMacros.IsValid` _returnvalue
              (:`Is Valid`
                (`/Game/RuinBot/BluePrints/DoorDamageTrigger.DamageTaken` _returnvalue (`self.DamageType`)))
              (:`Is Not Valid`
                _))
            (`/Engine/EditorBlueprintResources/StandardMacros.IsValid` self
              (:`Is Valid`
                (if (not (`self.Piercing`))
                  (`self.K2_DestroyActor` self)))))
          (:`else`))))))

(event `ReAim`
  (if (`self.Homing?`)
    (`self.K2_SetActorRotation` (`KismetMathLibrary.FindLookAtRotation` (`self.K2_GetActorLocation` self) (`SceneComponent.K2_GetComponentLocation` (`self.HomingTarget`))))
    (`ProjectileMovementComponent.SetVelocityInLocalSpace` (`self.ProjectileMovement`) (3000.0 0.0 0.0))))

(event `self.ReceiveHit`
  (params (MyComp :type "PrimitiveComponent Object Reference") (Other :type "Actor Object Reference") (OtherComp :type "PrimitiveComponent Object Reference") (bSelfMoved :type Boolean) (HitLocation :type "Vector Structure") (HitNormal :type "Vector Structure") (NormalImpulse :type "Vector Structure") (Hit :type "HitResult Structure (by ref)"))
  (`self.Hit/Over` Other (`SceneComponent.GetForwardVector` (`self.SM_LaserMesh`)) HitLocation))

(fn `UserConstructionScript`)