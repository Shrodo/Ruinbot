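; Sniper laser projectile Blueprint whose own logic is purely visual setup, with an empty event graph.
; Its construction script runs the parent's, then creates a dynamic instance of the laser material on the laser mesh.
; It feeds hue, desaturation and color blend variables into that material and sets the point light's color from a separate variable.
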(fn `UserConstructionScript`
  (`parent.UserConstructionScript`)
  (bind _returnvalue (`PrimitiveComponent.CreateDynamicMaterialInstance` (`self.SM_LaserMesh`) 0 "/Game/RuinBot/TexMat/M_Laser1.M_Laser1" "None"))
  (`MaterialInstanceDynamic.SetScalarParameterValue` _returnvalue "Hue" (`self.Hue`))
  (`MaterialInstanceDynamic.SetScalarParameterValue` _returnvalue "Desaturation" (`self.Desaturation`))
  (`MaterialInstanceDynamic.SetScalarParameterValue` _returnvalue "ColorBlend" (`self.ColorBlend`))
  (`LightComponent.SetLightColor` (`self.PointLight`) (`self.LightColor`) true))