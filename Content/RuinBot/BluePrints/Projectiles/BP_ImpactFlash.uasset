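; A short-lived impact flash actor, stored with the RuinBot projectiles, that lights its surroundings briefly and then removes itself.
; On BeginPlay it applies a dynamic LF_ImpactFlash material as the point light's light function and starts two timers.
; Tick fades the FlashColor parameter by the cubed remaining time of the light timer.
; That timer destroys the light first, and the longer timer then destroys the actor.
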(event `self.ReceiveBeginPlay`
  (bind _returnvalue (`KismetMaterialLibrary.CreateDynamicMaterialInstance` "/Game/RuinBot/TexMat/LF_ImpactFlash.LF_ImpactFlash"))
  (`LightComponent.SetLightFunctionMaterial` (`self.PointLight`) _returnvalue)
  (`KismetSystemLibrary.K2_SetTimerDelegate` (delegate `Kill`) 0.3)
  (bind _returnvalue_2 (`KismetSystemLibrary.K2_SetTimerDelegate` (delegate `Lightout`) 0.1)))

(event `Lightout`
  (`ActorComponent.K2_DestroyComponent` (`self.PointLight`)))

(event `self.ReceiveTick`
  (params (DeltaSeconds :type "Float (single-precision)"))
  (`/Engine/EditorBlueprintResources/StandardMacros.IsValid` (`self.PointLight`)
    (:`Is Valid`
      (`MaterialInstanceDynamic.SetVectorParameterValue` (stale `self.ReceiveBeginPlay` _returnvalue) "FlashColor" (* (`self.FlashColor`) (`KismetMathLibrary.MultiplyMultiply_FloatFloat` (`KismetSystemLibrary.K2_GetTimerRemainingTimeHandle` (stale `self.ReceiveBeginPlay` _returnvalue_2)) 3.0))))))

(event `Kill`
  (`/Engine/EditorBlueprintResources/StandardMacros.IsValid` self
    (:`Is Valid`
      (`self.K2_DestroyActor` self))))

(fn `UserConstructionScript`)