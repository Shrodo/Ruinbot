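; CryoTorch is an ice torch actor, filed under RuinBot projectiles, that deals periodic damage to whatever overlaps its mesh.
; A looping half-second timer started on BeginPlay fires IceAttack, which polls the actors overlapping TorchMesh and applies Damage to each, with itself as causer.
; The construction script gives the mesh a dynamic material instance tinted icy blue.
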(event `self.ReceiveBeginPlay`
  (`KismetSystemLibrary.K2_SetTimerDelegate` (delegate `IceAttack`) 0.5 true))

(event `IceAttack`
  (for _array_element (`PrimitiveComponent.GetOverlappingActors` (`self.TorchMesh`) "/Script/Engine.Actor")
    (`GameplayStatics.ApplyDamage` _array_element (`self.Damage`) null self)))

(fn `UserConstructionScript`
  (bind _returnvalue (`PrimitiveComponent.CreateDynamicMaterialInstance` (`self.TorchMesh`) 0 null "None"))
  (`MaterialInstanceDynamic.SetVectorParameterValue` _returnvalue "Color" (struct :`G` 0.263804 :`B` 0.432292 :`A` 1.0)))