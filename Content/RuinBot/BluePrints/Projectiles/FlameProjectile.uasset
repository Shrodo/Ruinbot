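; Flame projectile that deals fire damage on overlap or hit, with a random pitch/yaw spread set at construction.
; An attached FlameParticle follows it while a timeline scales the cube and drives its dynamic material color.
; Non-instigator contacts route through HitOver, which sets NPC death force, plays impact effects, applies damage and notifies DoorDamageTrigger components.
; Impact or timeline end deactivates the particle and destroys the projectile.
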(event `self.ReceiveBeginPlay`
  (bind _returnvalue (`|SpawnActorFromClass` "/Game/RuinBot/BluePrints/FlameParticle.FlameParticle_C" (`KismetMathLibrary.MakeTransform` (`SceneComponent.K2_GetComponentLocation` (`self.Cube`))) "AlwaysSpawn" "OverrideRootScale" null null))
  (bind _output_get (set `self.Flame2` _returnvalue))
  (`self.K2_AttachToActor` _output_get self "None" "SnapToTarget" "SnapToTarget" "SnapToTarget" true)
  (bind (_direction _flamesize _color) (`Timeline|FlameLife`)
    (:`Update`
      (bind _returnvalue_2 (* _flamesize (`self.FlameInitialSize`)))
      (`SceneComponent.SetWorldScale3D` (`self.Cube`) (`KismetMathLibrary.MakeVector` _returnvalue_2 _returnvalue_2 _returnvalue_2))
      (`MaterialInstanceDynamic.SetVectorParameterValue` (`self.FlameMat`) "Color" _color))
    (:`Finished`
      (`/Engine/EditorBlueprintResources/StandardMacros.IsValid` self
        (:`Is Valid`
          (`ActorComponent.Deactivate` (`/Game/RuinBot/BluePrints/FlameParticle.Flame` (`self.Flame2`)))
          (`self.K2_DestroyActor`))))))

(event `self.Cube.OnComponentBeginOverlap`
  (params (OverlappedComponent :type "PrimitiveComponent Object Reference") (OtherActor :type "Actor Object Reference") (OtherComp :type "PrimitiveComponent Object Reference") (OtherBodyIndex :type Integer) (bFromSweep :type Boolean) (SweepResult :type "HitResult Structure (by ref)"))
  (`self.Hit/Over` OtherActor (`SceneComponent.GetForwardVector` (`self.Cube`)) SweepResult_ImpactPoint))

(event `Hit/Over`
  (params (Other :type "Actor Object Reference") (HitNormal :type "Vector Structure") (HitLoc :type "Vector Structure"))
  (bind _returnvalue (`self.GetComponentByClass` Other "/Game/RuinBot/BluePrints/DoorDamageTrigger.DoorDamageTrigger_C"))
  (`/Engine/EditorBlueprintResources/StandardMacros.IsValid` Other
    (:`Is Valid`
      (if (not (== Other (`self.GetInstigator`)))
        (bind _asnpc_char (cast `/Game/RuinBot/AI/NPC_Char` Other)
          (:`then`
            (set `/Game/RuinBot/AI/NPC_Char.DeathForceVec` HitNormal _asnpc_char))
          (:`CastFailed`
            _))
        (`GameplayStatics.PlaySoundAtLocation` "/Engine/VREditor/Sounds/UI/Drop_Item_From_ContentBrowser.Drop_Item_From_ContentBrowser" HitLoc (struct) 1.0 (`KismetMathLibrary.RandomFloatInRange` 0.7 1.3) 0.0 null null null)
        (`|SpawnActorFromClass` (`self.ImpactBP`) (`KismetMathLibrary.MakeTransform` (.location (`SceneComponent.K2_GetComponentToWorld` (`self.Cube`))) (.rotation (`SceneComponent.K2_GetComponentToWorld` (`self.Cube`)))) "AlwaysSpawn" "OverrideRootScale" null null)
        (`GameplayStatics.ApplyDamage` Other (`self.Damage`) null self "/Game/RuinBot/BluePrints/BP_FireDamage.BP_FireDamage_C")
        (`/Engine/EditorBlueprintResources/StandardMacros.IsValid` _returnvalue
          (:`Is Valid`
            (`/Game/RuinBot/BluePrints/DoorDamageTrigger.DamageTaken` _returnvalue (`self.DamageType`)))
          (:`Is Not Valid`
            _))
        (`/Engine/EditorBlueprintResources/StandardMacros.IsValid` self
          (:`Is Valid`
            (`ActorComponent.Deactivate` (`/Game/RuinBot/BluePrints/FlameParticle.Flame` (`self.Flame2`)))
            (`self.K2_DestroyActor`)))))))

(event `self.ReceiveHit`
  (params (MyComp :type "PrimitiveComponent Object Reference") (Other :type "Actor Object Reference") (OtherComp :type "PrimitiveComponent Object Reference") (bSelfMoved :type Boolean) (HitLocation :type "Vector Structure") (HitNormal :type "Vector Structure") (NormalImpulse :type "Vector Structure") (Hit :type "HitResult Structure (by ref)"))
  (`self.Hit/Over` Other (`SceneComponent.GetForwardVector` (`self.Cube`)) HitLocation))

(fn `UserConstructionScript`
  (`self.K2_AddActorLocalRotation` self (`KismetMathLibrary.MakeRotator` 0.0 (`KismetMathLibrary.RandomFloatInRange` -10.0 10.0) (`KismetMathLibrary.RandomFloatInRange` -10.0 10.0)) false false)
  (`SceneComponent.K2_SetWorldRotation` :`self` (`self.Cube`))
  (bind _returnvalue (`PrimitiveComponent.CreateDynamicMaterialInstance` (`self.Cube`) 0 null "None"))
  (set `self.FlameMat` _returnvalue))