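; BP_sonarwave is a short-lived sonar pulse actor that expands from its spawn point and alerts objects it reaches.
; The PulseFade timeline drives radius and opacity on the SonarBlendable material, fades the sphere material and grows SonarOverlapVol to match.
; Overlapped actors are notified through their SonarNotice and MagneticObject components.
; Timer-based scaling and HUD notice logic remain in the graph but never run.
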(event `self.ReceiveBeginPlay`
  (bind _sonarblendable (`self.SonarBlendable`))
  (`MaterialInstanceDynamic.SetVectorParameterValue` (`self.SonarBlendable`) "RadarPosition" (`KismetMathLibrary.Conv_VectorToLinearColor` (`SceneComponent.K2_GetComponentLocation` (`self.Sphere`))))
  (`self.SetLifeSpan` (`self.Lifespan1`))
  (bind (_direction _opacity _bubblesize) (`Timeline|PulseFade` :!via `PlayFromStart`)
    (:`Update`
      (`MaterialInstanceDynamic.SetScalarParameterValue` _sonarblendable "RadarOpac" _opacity)
      (bind _returnvalue (* _bubblesize 4500.0))
      (`MaterialInstanceDynamic.SetScalarParameterValue` _sonarblendable "RadarRadius" _returnvalue)
      (`MeshComponent.SetScalarParameterValueOnMaterials` (`self.Sphere`) "Opac" _opacity)
      (`SphereComponent.SetSphereRadius` (`self.SonarOverlapVol`) _returnvalue true)
      (`SphereComponent.SetSphereRadius` (`self.SonarOverlapVol`) _returnvalue true))))

(event `Null`)

(event `Unfind`)

(event `Unnotice`)

(event `self.ReceiveTick`
  (params (DeltaSeconds :type "Float (single-precision)")))

(event `self.SonarOverlapVol.OnComponentBeginOverlap`
  (params (OverlappedComponent :type "PrimitiveComponent Object Reference") (OtherActor :type "Actor Object Reference") (OtherComp :type "PrimitiveComponent Object Reference") (OtherBodyIndex :type Integer) (bFromSweep :type Boolean) (SweepResult :type "HitResult Structure (by ref)"))
  (bind _returnvalue (`self.GetComponentByClass` OtherActor "/Game/RuinBot/BluePrints/MagneticObject.MagneticObject_C"))
  (bind _returnvalue_2 (`self.GetComponentByClass` OtherActor "/Game/RuinBot/BluePrints/SonarNotice.SonarNotice_C"))
  (`|ExecutionSequence`
    (:`then_0`
      (`/Engine/EditorBlueprintResources/StandardMacros.IsValid` _returnvalue_2
        (:`Is Valid`
          (`/Game/RuinBot/BluePrints/SonarNotice.Overlap` _returnvalue_2 self null))))
    (:`then_1`
      (`/Engine/EditorBlueprintResources/StandardMacros.IsValid` _returnvalue
        (:`Is Valid`
          (`/Game/RuinBot/BluePrints/MagneticObject.SonarOverlap` _returnvalue))))))

(fn `UserConstructionScript`
  (bind _returnvalue (`PrimitiveComponent.CreateDynamicMaterialInstance` (`self.Sphere`) 0 null "None"))
  (`PrimitiveComponent.SetMaterial` (`self.StaticMesh`) 0 _returnvalue)
  (`PrimitiveComponent.SetMaterial` (`self.StaticMesh1`) 0 _returnvalue))