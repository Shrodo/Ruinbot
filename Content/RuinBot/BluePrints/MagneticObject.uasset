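; MagneticObject is a component that lets its owning actor be found by sonar and moved by a magnet along a list of locations.
; A sonar overlap plays a sound, enables custom depth and shows a timed HUD notice.
; MagnetMove locks the object and lerps it point to point with timers, consuming trail actors.
; A scaled box trace checks each segment, and a hit turns remaining trails red, ends the move and clears them.
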(event `self.ReceiveBeginPlay`
  (bind _returnvalue (`Actor.GetComponentByClass` (`self.Actor`) "/Script/Engine.StaticMeshComponent"))
  (set `self.Actor` (`self.GetOwner`))
  (bind _staticmesh (`StaticMeshComponent.StaticMesh` _returnvalue)
    (:`then`
      (set `self.CollisionMesh` _staticmesh)
      (set `self.WorldTF` (`SceneComponent.K2_GetComponentToWorld` _returnvalue))
      (bind _asbp_ruin_bot_hud (cast `/Game/RuinBot/BluePrints/HUD/BP_RuinBotHUD` (`PlayerController.GetHUD` (`GameplayStatics.GetPlayerController` 0)))))
    (:`else`)))

(event `SonarOverlap`
  (if (not (`self.Found?`))
    (bind _result (`/Game/RuinBot/BluePrints/HUD/BP_RuinBotHUD.Notice Object` (stale `self.ReceiveBeginPlay` _asbp_ruin_bot_hud) (`self.Actor`) (`self.NoticeColor`) (0.0 0.0) (`self.NoticeOffset`) (`GameplayStatics.GetPlayerController` 0) (`self.NoticeDuration`) null null ""))
    (bind _asstatic_mesh_actor (cast `StaticMeshActor` (`self.Actor`))
      (:`then`
        (bind _staticmeshcomponent (`StaticMeshActor.StaticMeshComponent` _asstatic_mesh_actor)
          (:`then`
            (`PrimitiveComponent.SetRenderCustomDepth` _staticmeshcomponent true))
          (:`else`
            _)))
      (:`CastFailed`
        _))
    (`GameplayStatics.PlaySoundAtLocation` "/Game/RuinBot/Audio/Sonar4.Sonar4" (`SceneComponent.K2_GetComponentLocation` (`Actor.RootComponent` (`self.Actor`))) (struct) 2.0 (`KismetMathLibrary.RandomFloatInRange` 0.95 1.05) 0.0 null null null)
    (set `self.Found?` true)
    (`KismetSystemLibrary.K2_SetTimerDelegate` (delegate `Unfind`) (`self.NoticeDuration`))))

(event `Unfind`
  (set `self.Found?` false)
  (`self.Unnotice`))

(event `Unnotice`
  (`/Game/RuinBot/BluePrints/HUD/BP_RuinBotHUD.DestroyWidgetObj` (stale `self.ReceiveBeginPlay` _asbp_ruin_bot_hud) (stale `SonarOverlap` _result)))

(event `MagnetMove`
  (params (LocationsList :type "Array of Vector Structure") (Trails :type "Array of /Game/RuinBot/BluePrints/MagMoverTrail Object Reference"))
  (bind _moveslist (`self.MovesList`))
  (bind _trails (`self.Trails`))
  (if (> (`KismetArrayLibrary.Array_Length` LocationsList) 1)
    (set `self.Locked` true)
    (bind _output_get (set `self.MovesList` LocationsList))
    (set `self.Trails` Trails)
    (set `self.Moves` (- (`KismetArrayLibrary.Array_Length` _output_get) 1))
    (`self.OneMove`)
    (else
      (set `self.Trails` Trails)
      (for _array_element _trails :!label _label
        (`/Engine/EditorBlueprintResources/StandardMacros.IsValid` _array_element
          (:`Is Valid`
            (`Actor.K2_DestroyActor` _array_element))))
      (`KismetArrayLibrary.Array_Clear` _trails)
      (`KismetArrayLibrary.Array_Resize` _trails)
      (`KismetArrayLibrary.Array_Clear` _moveslist)
      (`KismetArrayLibrary.Array_Resize` _moveslist)
      (set `self.Moves` 0)
      (set `self.CurrentMove` 0)
      (set `self.Locked` false))))

(event `OneMove`
  (bind _currentmove (`self.CurrentMove`))
  (bind _moveslist (`self.MovesList`))
  (bind _currentmove_2 (`self.CurrentMove`))
  (bind _moverlocationoffset (`self.MoverLocationOffset`))
  (bind _moveslist_2 (`self.MovesList`))
  (bind (_worldtf_location _worldtf_rotation _worldtf_scale) (`KismetMathLibrary.BreakTransform` (`self.WorldTF`)))
  (bind _currentmove_3 (`self.CurrentMove`))
  (bind _output (`|GetArrayItem` (`self.Trails`) _currentmove_3))
  (bind _output_2 (`|GetArrayItem` _moveslist (+ _currentmove 1)))
  (bind (_returnvalue_origin _returnvalue_boxextent) (`KismetMathLibrary.BreakBoxSphereBounds` (`StaticMesh.GetBounds` (`StaticMeshComponent.StaticMesh` (`Actor.GetComponentByClass` (`self.Actor`) "/Script/Engine.StaticMeshComponent")))))
  (if (>= (`self.CurrentMove`) (`self.Moves`))
    (`KismetSystemLibrary.K2_ClearAndInvalidateTimerHandle` (stale `OneMove` _returnvalue_2) :!label _label_2)
    (`KismetSystemLibrary.K2_ClearAndInvalidateTimerHandle` (stale `OneMove` _returnvalue_3))
    (`Actor.K2_SetActorLocation` (`self.Actor`) (+ (`|GetArrayItem` (stale `MagnetMove` _output_get) (`self.Moves`)) (`self.MoverLocationOffset`)) false false)
    (set `self.WorldTF` (`SceneComponent.K2_GetComponentToWorld` (`Actor.GetComponentByClass` (`self.Actor`) "/Script/Engine.StaticMeshComponent")))
    (goto _label)
    (else
      (bind (_outhit _returnvalue) (`KismetSystemLibrary.BoxTraceSingle` (`KismetMathLibrary.VLerp` (`|GetArrayItem` _moveslist _currentmove) _output_2 0.3) _output_2 (* _returnvalue_boxextent _worldtf_scale (0.8 0.8 0.8)) (struct) "TraceTypeQuery1" false (`|MakeArray` (`self.Actor`))))
      (if _returnvalue
        (`self.CutoffPath`)
        (goto _label_2)
        (else
          (bind _returnvalue_2 (`KismetSystemLibrary.K2_SetTimerDelegate` (delegate `UpdateMove`) 0.01 true))
          (bind _returnvalue_3 (`KismetSystemLibrary.K2_SetTimer` null "MoveDuration" 2.0))
          (set `self.Location1` (+ (`|GetArrayItem` _moveslist_2 _currentmove_2) _moverlocationoffset))
          (set `self.Location2` (+ (`|GetArrayItem` _moveslist_2 (+ _currentmove_2 1)) _moverlocationoffset))
          (`/Engine/EditorBlueprintResources/StandardMacros.IsValid` _output
            (:`Is Valid`
              (`Actor.K2_DestroyActor` _output)
              (set `self.CurrentMove` (+ _currentmove_3 1)))))))))

(event `UpdateMove`
  (bind _returnvalue (`KismetSystemLibrary.K2_GetTimerElapsedTimeHandle` (stale `OneMove` _returnvalue_3)))
  (`Actor.K2_SetActorLocation` (`self.Actor`) (`KismetMathLibrary.VLerp` (`self.Location1`) (`self.Location2`) (/ _returnvalue (+ _returnvalue (`KismetSystemLibrary.K2_GetTimerRemainingTimeHandle` (stale `OneMove` _returnvalue_3))))) false false))

(event `SetMoverOffset`
  (params (NewParam :type "Vector Structure"))
  (set `self.MoverLocationOffset` NewParam))

(event `MoveDuration`
  (`self.OneMove`))

(event `ClearTimers`
  (`KismetSystemLibrary.K2_ClearAndInvalidateTimerHandle` (stale `OneMove` _returnvalue_2))
  (`KismetSystemLibrary.K2_ClearAndInvalidateTimerHandle` (stale `OneMove` _returnvalue_3)))

(event `CutoffPath`
  (set `self.Moves` (`self.CurrentMove`))
  (for _array_element (`self.Trails`)
    (`/Engine/EditorBlueprintResources/StandardMacros.IsValid` _array_element
      (:`Is Valid`
        (`MeshComponent.SetVectorParameterValueOnMaterials` (`/Game/RuinBot/BluePrints/MagMoverTrail.Cube` _array_element) "color" (`KismetMathLibrary.Conv_LinearColorToVector` (struct :`R` 0.796875 :`A` 1.0)))))))