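; BP_Hideable is a component that fades its owner's static meshes out and back in on trigger calls.
; On BeginPlay it creates dynamic materials for the meshes of the owner and its listed Children.
; TriggerHide records each trigger, and TriggerShow requests a show only once none remain.
; Tick steps each material's "Opac" parameter toward MinOpac or 1, turning mesh visibility off at the minimum and on when showing.
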(event `self.ReceiveTick`
  (params (DeltaSeconds :type "Float (single-precision)"))
  (bind _shouldhide (`self.ShouldHide`))
  (if (or _shouldhide (`self.ShouldShow`))
    (`self.UpdateVis` (* DeltaSeconds (`self.FadeSpeed`)) _shouldhide)))

(event `self.ReceiveBeginPlay`
  (bind _children (`self.Children`))
  (bind _returnvalue (`Actor.K2_GetComponentsByClass` (`self.GetOwner`) "/Script/Engine.StaticMeshComponent"))
  (if (`KismetArrayLibrary.Array_IsValidIndex` _returnvalue)
    (bind _output_get (set `self.Meshes` _returnvalue))
    (for _array_element _output_get
      (bind _returnvalue_2 (`MeshComponent.GetMaterials` _array_element))
      (if (`KismetArrayLibrary.Array_IsValidIndex` _returnvalue_2)
        (for (_array_element_2 _array_index) _returnvalue_2
          (bind _returnvalue_3 (`PrimitiveComponent.CreateDynamicMaterialInstance` _array_element _array_index _array_element_2 "None"))
          (`KismetArrayLibrary.Array_Add` (`self.HideMats`) _returnvalue_3))))
    (if (`KismetArrayLibrary.Array_IsValidIndex` _children)
      (for _array_element_3 _children
        (for _array_element_4 (`Actor.K2_GetComponentsByClass` _array_element_3 "/Script/Engine.StaticMeshComponent")
          (`KismetArrayLibrary.Array_AddUnique` (`self.Meshes`) _array_element_4)
          (for (_array_element_5 _array_index_2) (`MeshComponent.GetMaterials` _array_element_4)
            (bind _returnvalue_4 (`PrimitiveComponent.CreateDynamicMaterialInstance` _array_element_4 _array_index_2 _array_element_5 "None"))
            (`KismetArrayLibrary.Array_Add` (`self.HideMats`) _returnvalue_4)))))))

(fn `Hide`
  (params (`Trigger?` :type Boolean))
  (if (== `Trigger?` (`self.TriggerHide?`))
    (set `self.ShouldHide` true)
    (set `self.ShouldShow` false)))

(fn `Show`
  (params (`Trigger?` :type Boolean))
  (if (== `Trigger?` (`self.TriggerHide?`))
    (set `self.ShouldShow` true)
    (set `self.ShouldHide` false)))

(fn `TriggerHide`
  (params (Trigger :type "/Game/RuinBot/BluePrints/LocationMarker Object Reference"))
  (`KismetArrayLibrary.Array_AddUnique` (`self.HideTriggers`) Trigger)
  (`self.Hide` true))

(fn `TriggerShow`
  (params (Trigger :type "/Game/RuinBot/BluePrints/LocationMarker Object Reference"))
  (bind _hidetriggers (`self.HideTriggers`))
  (`KismetArrayLibrary.Array_RemoveItem` _hidetriggers Trigger)
  (if (== (`KismetArrayLibrary.Array_Length` _hidetriggers) 0)
    (`self.Show` true)))

(fn `UpdateVis`
  (params (Amount :type "Float (double-precision)") (ShouldHide :type Boolean))
  (bind _minopac (`self.MinOpac`))
  (for _array_element (`self.HideMats`)
    (bind _returnvalue (`MaterialInstanceDynamic.K2_GetScalarParameterValue` _array_element "Opac"))
    (if ShouldHide
      (bind _returnvalue_2 (- _returnvalue Amount))
      (bind _returnvalue_3 (not (<= _returnvalue_2 _minopac)))
      (if _returnvalue_3
        (`MaterialInstanceDynamic.SetScalarParameterValue` _array_element "Opac" _returnvalue_2)
        (set `self.ShouldHide` _returnvalue_3)
        (else
          (`MaterialInstanceDynamic.SetScalarParameterValue` _array_element "Opac" _minopac)
          (for _array_element_2 (`self.Meshes`)
            (`SceneComponent.SetVisibility` _array_element_2 false false))))
      (else
        (for _array_element_3 (`self.Meshes`)
          (`SceneComponent.SetVisibility` _array_element_3 true false))
        (bind _returnvalue_4 (+ _returnvalue Amount))
        (bind _returnvalue_5 (not (>= _returnvalue_4 1.0)))
        (if _returnvalue_5
          (`MaterialInstanceDynamic.SetScalarParameterValue` _array_element "Opac" _returnvalue_4)
          (set `self.ShouldShow` _returnvalue_5)
          (else
            (`MaterialInstanceDynamic.SetScalarParameterValue` _array_element "Opac" 1.0)))))))