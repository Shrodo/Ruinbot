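; SpaceHUD is the HUD for the space controller, managing the main HUD, planet, quick menu, on-foot map menu and space map widgets.
; BeginPlay caches the owning BP_SpaceController and adds all five widgets to the viewport up front.
; Tick polls the controller's state flags to toggle visibility, swapping planet and main HUD and hiding the space map in planet view or on foot.
; Two events forward planet attributes and minimap creation to their widgets.
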(event `NotifyMinimap`
  (`/Game/RuinBot/BluePrints/HUD/OF_MapMenu_UI.MakeMap` (stale `self.ReceiveBeginPlay` _returnvalue_4)))

(event `PlanetAttributes`
  (params (Type :type String) (PlanetName :type Name))
  (`/Game/RuinBot/BluePrints/HUD/Planet_UI.PlanetAttr` (stale `self.ReceiveBeginPlay` _returnvalue_2) Type PlanetName))

(event `self.ReceiveBeginPlay`
  (bind _asbp_space_controller (cast `/Game/Blueprints/BP_SpaceController` (`self.GetOwningPlayerController`)))
  ;[1 1 1] HUD creation
  (bind _returnvalue (`WidgetBlueprintLibrary.Create` "/Game/RuinBot/BluePrints/HUD/UMG_HUD.UMG_HUD_C")) ; This chooses which UMG object to use as the hud
  (`UserWidget.AddToViewport` _returnvalue 0) ; This
  (bind _returnvalue_2 (`|CreateWidget` "/Game/RuinBot/BluePrints/HUD/Planet_UI.Planet_UI_C"))
  (`UserWidget.AddToViewport` _returnvalue_2 0) ; This
  (bind _returnvalue_3 (`|CreateWidget` "/Game/RuinBot/BluePrints/HUD/QuickMenu_UI.QuickMenu_UI_C"))
  (`UserWidget.AddToViewport` _returnvalue_3 0)
  (bind _returnvalue_4 (`|CreateWidget` "/Game/RuinBot/BluePrints/HUD/OF_MapMenu_UI.OF_MapMenu_UI_C"))
  (`UserWidget.AddToViewport` _returnvalue_4 0)
  (bind _returnvalue_5 (`|CreateWidget` "/Game/RuinBot/BluePrints/HUD/UI_SpaceMap.UI_SpaceMap_C"))
  (`UserWidget.AddToViewport` _returnvalue_5 0))

(event `self.ReceiveTick`
  (params (DeltaSeconds :type "Float (single-precision)"))
  (`|ExecutionSequence`
    (:`then_0`
      (bind _planetview (`/Game/Blueprints/BP_SpaceController.PlanetView` (stale `self.ReceiveBeginPlay` _asbp_space_controller)))
      (if _planetview
        (`Widget.SetVisibility` (stale `self.ReceiveBeginPlay` _returnvalue_2) "Visible")
        (`Widget.SetVisibility` (stale `self.ReceiveBeginPlay` _returnvalue) "Hidden")
        (else
          (`Widget.SetVisibility` (stale `self.ReceiveBeginPlay` _returnvalue) "Visible")
          (`Widget.SetVisibility` (stale `self.ReceiveBeginPlay` _returnvalue_2) "Hidden"))))
    (:`then_1`
      (if (`/Game/Blueprints/BP_SpaceController.QuickMenu_g` (stale `self.ReceiveBeginPlay` _asbp_space_controller))
        (`Widget.SetVisibility` (stale `self.ReceiveBeginPlay` _returnvalue_3) "Visible")
        (else
          (`Widget.SetVisibility` (stale `self.ReceiveBeginPlay` _returnvalue_3) "Hidden"))))
    (:`then_2`
      (if (`/Game/Blueprints/BP_SpaceController.MapMenu` (stale `self.ReceiveBeginPlay` _asbp_space_controller))
        (`Widget.SetVisibility` (stale `self.ReceiveBeginPlay` _returnvalue_4) "Visible")
        (else
          (`Widget.SetVisibility` (stale `self.ReceiveBeginPlay` _returnvalue_4) "Hidden"))))
    (:`then_3`
      (if (or _planetview (`/Game/Blueprints/BP_SpaceController.OnFoot` (stale `self.ReceiveBeginPlay` _asbp_space_controller)))
        (`Widget.SetVisibility` (stale `self.ReceiveBeginPlay` _returnvalue_5) "Hidden")
        (else
          (`Widget.SetVisibility` (stale `self.ReceiveBeginPlay` _returnvalue_5) "Visible"))))))

(fn `UserConstructionScript`)