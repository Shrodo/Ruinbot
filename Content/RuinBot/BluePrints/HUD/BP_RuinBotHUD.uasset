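; BP_RuinBotHUD is RuinBot's HUD, creating and managing widgets for health, prompts, menus, console readouts, wave announcements and death or win screens.
; It pre-creates three weapon wheels and passes selections to the player controller on close.
; NoticeObject attaches tagged widget components to world actors as markers.
; It also runs terrain editing, tracing from the mouse to edit BP_TerrainMaker tiles and relaying resize, save and load between editor widget and terrain.
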(event `self.ReceiveBeginPlay`
  (bind _returnvalue (`GameplayStatics.GetPlayerController` 0))
  (bind _returnvalue_2 (`|CreateWidget` "/Game/RuinBot/BluePrints/HUD/W_Prompts.W_Prompts_C" _returnvalue))
  (`UserWidget.AddToViewport` _returnvalue_2 0)
  (bind _returnvalue_3 (`|CreateWidget` "/Game/RuinBot/BluePrints/HUD/W_HealthReadout.W_HealthReadout_C" _returnvalue))
  (`UserWidget.AddToViewport` _returnvalue_3 1)
  (bind _returnvalue_4 (`|CreateWidget` "/Game/RuinBot/BluePrints/HUD/W_StartScreen.W_StartScreen_C" _returnvalue))
  (set `self.StartMenu` _returnvalue_4)
  (bind _asbp_ruin_bot_player_controller (cast `/Game/RuinBot/BluePrints/BP_RuinBotPlayerController` (`GameplayStatics.GetPlayerController` 0)))
  (set `self.RBController` _asbp_ruin_bot_player_controller)
  (set `self.RBCharacter` (`GameplayStatics.GetPlayerCharacter` 0))
  (bind _returnvalue_5 (`|CreateWidget` "/Game/RuinBot/BluePrints/HUD/WeaponWheel.WeaponWheel_C"))
  (set `self.PrimWheelWJT` _returnvalue_5)
  (bind _returnvalue_6 (`|CreateWidget` "/Game/RuinBot/BluePrints/HUD/WeaponWheel.WeaponWheel_C"))
  (set `self.SecWheelWJT` _returnvalue_6)
  (bind _returnvalue_7 (`|CreateWidget` "/Game/RuinBot/BluePrints/HUD/WeaponWheel.WeaponWheel_C"))
  (set `self.GadgetWheelWJT` _returnvalue_7))

(event `HUD_XproGo`
  (params (`Default Text?` :type Boolean :default true) (SubText :type String) (ButtonID :type Integer) (`Gamepad?` :type Boolean) (Key :type String))
  (bind _prompt (`/Game/RuinBot/BluePrints/HUD/W_Prompts.X Prompt Go1` (stale `self.ReceiveBeginPlay` _returnvalue_2) `Default Text?` SubText ButtonID `Gamepad?` Key))
  (bind _currentprompt (`self.CurrentPrompt`)
    (:`then`
      (`Widget.RemoveFromParent` _currentprompt)
      (set `self.CurrentPrompt` _prompt))
    (:`else`)))

(event `HUD_XproStop`
  (`/Game/RuinBot/BluePrints/HUD/W_Prompts.X Prompt Stop` (stale `self.ReceiveBeginPlay` _returnvalue_2)))

(event `Unnotice All`
  (bind _foundwidgets (`WidgetBlueprintLibrary.GetAllWidgetsOfClass` "/Game/RuinBot/BluePrints/HUD/W_Notice.W_Notice_C" false))
  (for _array_element _foundwidgets
    (`/Engine/EditorBlueprintResources/StandardMacros.IsValid` _array_element
      (:`Is Valid`
        (`Widget.RemoveFromParent` _array_element)))))

(event `Healthupdate`
  (params (HealthFrac :type "Float (double-precision)"))
  (`/Engine/EditorBlueprintResources/StandardMacros.IsValid` (stale `self.ReceiveBeginPlay` _returnvalue_3)
    (:`Is Valid`
      (`/Game/RuinBot/BluePrints/HUD/W_HealthReadout.Hupdate` (stale `self.ReceiveBeginPlay` _returnvalue_3) HealthFrac))))

(event `AllowConsoleSkip`
  (`/Game/RuinBot/BluePrints/HUD/W_Console.AllowSkip` (`self.CurConsole`)))

(event `LoadTerrain`
  (params (LoadSlot :type String))
  (bind _terraineditobject (`self.TerrainEditObject`))
  ;[1 1 1] TerrainEdit
  (`/Game/Spirate/Blueprints/BP_TerrainMaker.LoadTerrain` _terraineditobject LoadSlot true)
  (`/Game/RuinBot/BluePrints/HUD/W_TerrainEdit.SetSizeSpinners` (`self.TerrainEditWidget`) (`/Game/Spirate/Blueprints/BP_TerrainMaker.TerrainSizeX` _terraineditobject) (`/Game/Spirate/Blueprints/BP_TerrainMaker.TerrainSizeY` _terraineditobject)))

(event `ClearConsole`
  (bind _foundwidgets (`WidgetBlueprintLibrary.GetAllWidgetsOfClass` "/Game/RuinBot/BluePrints/HUD/W_Console.W_Console_C"))
  (for _array_element _foundwidgets
    (`/Engine/EditorBlueprintResources/StandardMacros.IsValid` _array_element
      (:`Is Valid`
        (`GameplayStatics.PlaySound2D` "/Game/RuinBot/Audio/ConsoleClick.ConsoleClick" 1.0 1.0 0.0 null null)
        (`Widget.RemoveFromParent` _array_element)))))

(event `SaveTerrain`
  (params (SaveSlot :type String))
  (bind _terraineditobject (`self.TerrainEditObject`))
  ;[1 1 1] TerrainEdit
  (`/Game/Spirate/Blueprints/BP_TerrainMaker.SaveTerrain` _terraineditobject SaveSlot)
  (`/Game/RuinBot/BluePrints/HUD/W_TerrainEdit.UpdateLoadSlots` (stale `EditEnable` _output_get) (`/Game/Spirate/Blueprints/BP_TerrainMaker.ExistingSlots` _terraineditobject)))

(event `PauseMenu`
  (params (Screen :type "UserWidget Object Reference"))
  (`UserWidget.AddToViewport` Screen 0)
  (set `PlayerController.bShowMouseCursor` true (`GameplayStatics.GetPlayerController` 0)))

(event `InteractionMenu`
  (params (SpawnPad :type "/Game/RuinBot/BluePrints/EnemySpawnPad Object Reference"))
  (`/Engine/EditorBlueprintResources/StandardMacros.IsValid` SpawnPad
    (:`Is Valid`
      (`GameplayStatics.SetGamePaused` true)
      (bind _returnvalue (`|CreateWidget` "/Game/RuinBot/BluePrints/HUD/w_EnemySpawner.W_EnemySpawner_C" null SpawnPad))
      (bind _output_get (set `self.EnemySpawner` _returnvalue))
      (`UserWidget.AddToViewport` _output_get 0)
      (set `PlayerController.bShowMouseCursor` true (`GameplayStatics.GetPlayerController` 0)))))

(event `EditEnable`
  (bind _returnvalue (`GameplayStatics.GetPlayerController` 0))
  (bind _terraineditobject (`self.TerrainEditObject`))
  ;[1 1 1] TerrainEdit
  (set `PlayerController.bShowMouseCursor` true _returnvalue)
  (bind _returnvalue_2 (`|CreateWidget` "/Game/RuinBot/BluePrints/HUD/W_TerrainEdit.W_TerrainEdit_C" _returnvalue))
  (bind _output_get (set `self.TerrainEditWidget` _returnvalue_2))
  (`/Engine/EditorBlueprintResources/StandardMacros.IsValid` _terraineditobject
    (:`Is Valid`
      (`/Game/RuinBot/BluePrints/HUD/W_TerrainEdit.SetSizeSpinners` _output_get (`/Game/Spirate/Blueprints/BP_TerrainMaker.TerrainSizeX` _terraineditobject) (`/Game/Spirate/Blueprints/BP_TerrainMaker.TerrainSizeY` _terraineditobject)))
    (:`Is Not Valid`
      _))
  (`/Game/RuinBot/BluePrints/HUD/W_TerrainEdit.CastHUD` _output_get self)
  (`UserWidget.AddToViewport` _returnvalue_2 0))

(event `ExitInteractionMenu`
  (params (Widget :type "UserWidget Object Reference"))
  (`/Engine/EditorBlueprintResources/StandardMacros.IsValid` Widget
    (:`Is Valid`
      (`GameplayStatics.SetGamePaused` false)
      (cast `/Game/RuinBot/BluePrints/HUD/w_EnemySpawner` Widget
        (:`then`
          (set `self.EnemySpawner` null))
        (:`CastFailed`
          _))
      (`Widget.RemoveFromParent` Widget)
      (set `PlayerController.bShowMouseCursor` false (`GameplayStatics.GetPlayerController` 0)))))

(event `Unpause`
  (params (Screen :type "UserWidget Object Reference"))
  (`Widget.RemoveFromParent` Screen)
  (set `PlayerController.bShowMouseCursor` false (`GameplayStatics.GetPlayerController` 0)))

(event `EditDisable`
  ;[1 1 1] TerrainEdit
  (set `PlayerController.bShowMouseCursor` false (`GameplayStatics.GetPlayerController` 0))
  (`Widget.RemoveFromParent` (`self.TerrainEditWidget`))
  (set `self.TerrainEditWidget` null))

(event `Cancel`
  (`/Game/RuinBot/BluePrints/HUD/W_StartScreen.MenuCancel` (`self.StartMenu`)))

(event `EditClick`
  (bind _terraineditwidget (`self.TerrainEditWidget`))
  (bind (_worldlocation _worlddirection) (`PlayerController.DeprojectMousePositionToWorld` (`GameplayStatics.GetPlayerController` 0)))
  ;[1 1 1] TerrainEdit
  (bind _outhit (`KismetSystemLibrary.LineTraceSingle` :`Start` _worldlocation :`End` (+ _worldlocation (* _worlddirection 30000.0)) :`TraceChannel` "TraceTypeQuery1" :`DrawDebugType` "ForOneFrame"))
  (bind _asstatic_mesh_component (cast `StaticMeshComponent` (`.HitComponent` (`GameplayStatics.BreakHitResult` _outhit))))
  (bind _asbp_terrain_maker (cast `/Game/Spirate/Blueprints/BP_TerrainMaker` (`ActorComponent.GetOwner` _asstatic_mesh_component))
    (:`then`
      (bind _output_get (set `self.TerrainEditObject` _asbp_terrain_maker))
      (`/Engine/EditorBlueprintResources/StandardMacros.IsValid` _asbp_terrain_maker
        (:`Is Valid`
          (`/Game/RuinBot/BluePrints/HUD/W_TerrainEdit.SetSizeSpinners` (`self.TerrainEditWidget`) (`/Game/Spirate/Blueprints/BP_TerrainMaker.TerrainSizeX` _output_get) (`/Game/Spirate/Blueprints/BP_TerrainMaker.TerrainSizeY` _output_get))
          (`/Game/Spirate/Blueprints/BP_TerrainMaker.EditTile` _asbp_terrain_maker _asstatic_mesh_component (`/Game/RuinBot/BluePrints/HUD/W_TerrainEdit.CurElev` _terraineditwidget) (`/Game/RuinBot/BluePrints/HUD/W_TerrainEdit.ToolID?` _terraineditwidget) (`/Game/RuinBot/BluePrints/HUD/W_TerrainEdit.AddRamp?` _terraineditwidget))
          (`/Game/RuinBot/BluePrints/HUD/W_TerrainEdit.UpdateLoadSlots` (stale `EditEnable` _output_get) (`/Game/Spirate/Blueprints/BP_TerrainMaker.ExistingSlots` (`self.TerrainEditObject`))))
        (:`Is Not Valid`
          (`KismetSystemLibrary.PrintString` "Invalid TerrainObject"))))
    (:`CastFailed`
      (`KismetSystemLibrary.PrintString` "Hello"))))

(event `NewWave`
  (params (`Wave#` :type Integer))
  (bind _returnvalue (`|CreateWidget` "/Game/RuinBot/BluePrints/HUD/W_WaveAnnouncement.W_WaveAnnouncement_C" (`GameplayStatics.GetPlayerController` 0)))
  (`UserWidget.AddToViewport` _returnvalue 0)
  (`/Game/RuinBot/BluePrints/HUD/W_WaveAnnouncement.WaveCountdown` _returnvalue `Wave#`)
  (`KismetSystemLibrary.K2_SetTimer` null "CloseWaveTitle" 15.0))

(event `CloseWaveTitle`
  (`/Engine/EditorBlueprintResources/StandardMacros.IsValid` (stale `NewWave` _returnvalue)
    (:`Is Valid`
      (`Widget.RemoveFromParent` (stale `NewWave` _returnvalue)))))

(event `TerrainUpdate`
  (bind _terraineditobject (`self.TerrainEditObject`))
  ;[1 1 1] TerrainEdit
  (`/Engine/EditorBlueprintResources/StandardMacros.IsValid` _terraineditobject
    (:`Is Valid`
      (`/Game/Spirate/Blueprints/BP_TerrainMaker.ReInitUpdate` _terraineditobject))))

(event `Death`
  (params (`waves?` :type Boolean) (wave :type Integer))
  (bind _returnvalue (`|CreateWidget` "/Game/RuinBot/BluePrints/HUD/W_Dead.W_Dead_C" (`GameplayStatics.GetPlayerController` 0)))
  (`/Game/RuinBot/BluePrints/HUD/W_Dead.DeadText` _returnvalue wave `waves?`)
  (`UserWidget.AddToViewport` _returnvalue 0))

(event `Update Size`
  (params (X :type Integer) (Y :type Integer))
  ;[1 1 1] TerrainEdit
  (`/Game/Spirate/Blueprints/BP_TerrainMaker.ResizeTerrain` (`self.TerrainEditObject`) X Y))

(event `EndWin`
  (bind _returnvalue (`|CreateWidget` "/Game/RuinBot/BluePrints/HUD/W_EndScreen.W_EndScreen_C" (`GameplayStatics.GetPlayerController` 0)))
  (`UserWidget.AddToViewport` _returnvalue 0))

(event `PrimWheelScreen`
  (params (Upgrades :type "Array of Boolean") (OldSelection :type Integer))
  (bind _primwheelwjt (`self.PrimWheelWJT`))
  (`/Game/RuinBot/BluePrints/HUD/WeaponWheel.InitWheel` _primwheelwjt 0 OldSelection Upgrades false)
  (`UserWidget.AddToViewport` _primwheelwjt 0))

(event `SecWheelScreen`
  (params (Upgrades :type "Array of Boolean") (OldSelection :type Integer))
  (bind _secwheelwjt (`self.SecWheelWJT`))
  (`/Game/RuinBot/BluePrints/HUD/WeaponWheel.InitWheel` _secwheelwjt 1 OldSelection Upgrades false)
  (`UserWidget.AddToViewport` _secwheelwjt 0))

(event `GadgetWheelScreen`
  (params (Upgrades :type "Array of Boolean") (OldSelection :type Integer) (GadgetLock :type Boolean))
  (bind _gadgetwheelwjt (`self.GadgetWheelWJT`))
  (`/Game/RuinBot/BluePrints/HUD/WeaponWheel.InitWheel` _gadgetwheelwjt 2 OldSelection Upgrades GadgetLock)
  (`UserWidget.AddToViewport` _gadgetwheelwjt 0))

(event `CloseWheel`
  (params (Wheel :type "/Game/RuinBot/BluePrints/HUD/WeaponWheel Object Reference"))
  (`/Game/RuinBot/BluePrints/BP_RuinBotPlayerController.WheelSelection` (`self.RBController`) (`/Game/RuinBot/BluePrints/HUD/WeaponWheel.WheelType` Wheel) (`/Game/RuinBot/BluePrints/HUD/WeaponWheel.HighlightedItem` Wheel))
  (`Widget.RemoveFromParent` Wheel))

(fn `ConsoleReadout`
  (params (ReadoutText :type Text) (`Gamepad?` :type Boolean) (`CanSkip?` :type Boolean))
  (returns (NewParam :type "/Game/RuinBot/BluePrints/HUD/W_Console Object Reference"))
  (bind _returnvalue (`|CreateWidget` "/Game/RuinBot/BluePrints/HUD/W_Console.W_Console_C" (`GameplayStatics.GetPlayerController` 0)))
  (bind _output_get (set `self.CurConsole` _returnvalue))
  (`UserWidget.AddToViewport` _output_get 0)
  (`/Game/RuinBot/BluePrints/HUD/W_Console.Init_Console` _returnvalue ReadoutText `Gamepad?` `CanSkip?`)
  (return _returnvalue))

(fn `DestroyWidgetObj`
  (params (widget :type "WidgetComponent Object Reference"))
  (`/Engine/EditorBlueprintResources/StandardMacros.IsValid` widget
    (:`Is Valid`
      (`ActorComponent.K2_DestroyComponent` widget))))

(fn `Notice Object`
  (params (`Noticed Object` :type "Actor Object Reference") (NoticeColor :type "LinearColor Structure") (Size :type "Vector2D Structure") (Offset :type "Vector Structure") (OwningPlayer :type "PlayerController Object Reference") (Duration :type "Float (double-precision)") (Texture :type "Texture2D Object Reference") (Material :type "Material Object Reference") (Description :type Text))
  (returns (Result :type "WidgetComponent Object Reference"))
  (bind _returnvalue (`KismetStringLibrary.Conv_StringToName` (`KismetSystemLibrary.GetObjectName` `Noticed Object`)))
  (bind _returnvalue_2 (`AddComponent|NODE_AddWidgetComponent-1` :`self` (`self.RBCharacter`) :`RelativeTransform` (`KismetMathLibrary.MakeRelativeTransform` (`KismetMathLibrary.MakeTransform` (+ (`self.K2_GetActorLocation` `Noticed Object`) Offset) (struct) (1.0 1.0 1.0)) (`self.GetTransform` `Noticed Object`))))
  (bind _returnvalue_3 (`|CreateWidget` "/Game/RuinBot/BluePrints/HUD/W_Notice.W_Notice_C" OwningPlayer `Noticed Object` NoticeColor (select `bool` (!= Size (0.0 0.0)) :`false` (32.0 32.0) :`true` Size) Offset Duration Texture self _returnvalue Material Description))
  (`WidgetComponent.SetWidget` _returnvalue_2 _returnvalue_3)
  (set `ActorComponent.ComponentTags` (`|MakeArray` _returnvalue) _returnvalue_2)
  (`SceneComponent.K2_AttachToComponent` _returnvalue_2 (`Actor.RootComponent` `Noticed Object`) "None" "KeepRelative" "KeepRelative" "KeepRelative" true)
  (return _returnvalue_2))

(fn `UserConstructionScript`)