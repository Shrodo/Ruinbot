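; LocationMarker is a configurable box trigger whose LocType selects door, hideable, fall or level-load behaviour for overlapping players and NPCs.
; Doors and Hideables resolve from the parent actor, with player/NPC permission and blindness checks gating opening or hiding.
; Looping timers poll overlaps, rather than using EndOverlap, to close or reveal once the box clears.
; Fall calls the player's Fallout, LevelLoad stores DoorID before opening a level, and Camera only caches the player.
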(event `self.ReceiveBeginPlay`
  (bind _returnvalue (`self.GetAttachParentActor`))
  (bind _returnvalue_2 (`self.GetComponentByClass` _returnvalue "/Game/RuinBot/BluePrints/BP_Hideable.BP_Hideable_C"))
  (switch `/Game/RuinBot/BluePrints/LocationType` (`self.LocType`)
    (:`NewEnumerator0`
      (bind _asbp_door (cast `/Game/RuinBot/BluePrints/BP_Door` _returnvalue))
      (set `self.ParentDoor` _asbp_door))
    (:`NewEnumerator1`
      (`|ExecutionSequence`
        (:`then_0`
          (`/Engine/EditorBlueprintResources/StandardMacros.IsValid` _returnvalue
            (:`Is Valid`
              (`/Engine/EditorBlueprintResources/StandardMacros.IsValid` _returnvalue_2
                (:`Is Valid`
                  (set `self.Hideable` _returnvalue_2))))))
        (:`then_1`
          (`KismetSystemLibrary.Delay` 0.1)
          (`self.HideInitialize`))))
    (:`NewEnumerator2`
      (bind _asruin_bot_test_char (cast `/Game/RuinBot/Character/RuinBotTestChar` (`Controller.K2_GetPawn` (`GameplayStatics.GetPlayerController` 0))))
      (set `self.RBChar` _asruin_bot_test_char))))

(event `SetDoorOpenTimer`
  (`self.ParentDoor` :!label _label
    (:`then`
      (`KismetSystemLibrary.K2_SetTimer` null "OverlapTimeout" 5.0 true))
    (:`else`)))

(event `self.Box.OnComponentBeginOverlap`
  (params (OverlappedComponent :type "PrimitiveComponent Object Reference") (OtherActor :type "Actor Object Reference") (OtherComp :type "PrimitiveComponent Object Reference") (OtherBodyIndex :type Integer) (bFromSweep :type Boolean) (SweepResult :type "HitResult Structure (by ref)"))
  (bind _asruin_bot_test_char (cast `/Game/RuinBot/Character/RuinBotTestChar` OtherActor)
    (:`then`
      (`self.TriggerCondition` _asruin_bot_test_char null true true))
    (:`CastFailed`
      (bind _asnpc_char (cast `/Game/RuinBot/AI/NPC_Char` OtherActor))
      (`self.TriggerCondition` null _asnpc_char false true)))
  (`|ExecutionSequence`
    (:`then_0`
      (goto _label))
    (:`then_1`
      (`self.Hideable`
        (:`then`
          (`KismetSystemLibrary.K2_SetTimer` null "HideTimeOut" 1.0 true))
        (:`else`)))))

(fn `HideInitialize`
  (bind _hideable (`self.Hideable`)
    (:`then`
      (for _array_element (`PrimitiveComponent.GetOverlappingActors` (`self.Box`) null)
        (cast `/Game/RuinBot/Character/RuinBotTestChar` _array_element)
        (`/Game/RuinBot/BluePrints/BP_Hideable.TriggerHide` _hideable self)
        (`KismetSystemLibrary.K2_SetTimer` null "HideTimeOut" 1.0 true)
        (break)))
    (:`else`)))

(fn `HideTimeOut`
  (set `self.HoldHide` false)
  (for _array_element (`PrimitiveComponent.GetOverlappingActors` (`self.Box`) null)
    (cast `/Game/RuinBot/Character/RuinBotTestChar` _array_element
      (:`then`
        (if (`self.PlayerCanTrigger`)
          (set `self.HoldHide` true :!label _label)
          (break)
          (else
            (cast `/Game/RuinBot/AI/NPC_Char` _array_element :!label _label_2)
            (if (`self.NPCCanTrigger`)
              (goto _label)))))
      (:`CastFailed`
        (goto _label_2))))
  (if (not (`self.HoldHide`))
    (`KismetSystemLibrary.K2_ClearTimer` null "HideTimeOut")
    (bind _hideable (`self.Hideable`)
      (:`then`
        (`/Game/RuinBot/BluePrints/BP_Hideable.TriggerShow` _hideable self))
      (:`else`))))

(fn `OverlapTimeout`
  (for _array_element (`PrimitiveComponent.GetOverlappingActors` (`self.Box`) null)
    (cast `/Game/RuinBot/Character/RuinBotTestChar` _array_element
      (:`then`
        _)
      (:`CastFailed`
        (cast `/Game/RuinBot/AI/NPC_Char` _array_element)))
    (set `self.HoldDoor` true)
    (break))
  (if (`self.HoldDoor`)
    (set `self.HoldDoor` false)
    (else
      (`KismetSystemLibrary.K2_ClearTimer` null "OverlapTimeout")
      (`/Game/RuinBot/BluePrints/BP_Door.DoorClose` (`self.ParentDoor`)))))

(fn `TriggerCondition`
  (params (OverlapPlayer :type "/Game/RuinBot/Character/RuinBotTestChar Object Reference") (OverlapNPC :type "/Game/RuinBot/AI/NPC_Char Object Reference") (`Player?` :type Boolean) (`In/Out` :type Boolean))
  (switch `/Game/RuinBot/BluePrints/LocationType` (`self.LocType`)
    (:`NewEnumerator0`
      (if `Player?` :!label _label
        (if (`self.PlayerCanTrigger`)
          (if (`self.CheckBlind`)
            (if (== (`self.BlindValue`) (`/Game/RuinBot/Character/RuinBotTestChar.Blind?` OverlapPlayer))
              (if `In/Out` :!label _label_2
                (`|ExecutionSequence`
                  (:`then_0`
                    (bind _parentdoor (`self.ParentDoor`)
                      (:`then`
                        (`/Game/RuinBot/BluePrints/BP_Door.DoorOpen` _parentdoor))
                      (:`else`)))
                  (:`then_1`
                    (bind _hideable (`self.Hideable`)
                      (:`then`
                        (`/Game/RuinBot/BluePrints/BP_Hideable.TriggerHide` _hideable self))
                      (:`else`))))))
            (else
              (goto _label_2))))
        (elif (`self.NPCCanTrigger`)
          (goto _label_2))))
    (:`NewEnumerator1`
      (goto _label))
    (:`NewEnumerator3`
      (if `Player?`
        (`/Game/RuinBot/Character/RuinBotTestChar.Fallout` OverlapPlayer)
        (else
          (`/Engine/EditorBlueprintResources/StandardMacros.IsValid` OverlapNPC
            (:`Is Valid`
              (`self.K2_DestroyActor`))))))
    (:`NewEnumerator4`
      (if (and `Player?` `In/Out`)
        (bind _asbp_ruin_bot_gameinstance (cast `/Game/RuinBot/BluePrints/BP_RuinBotGameinstance` (`GameplayStatics.GetGameInstance`)))
        (set `/Game/RuinBot/BluePrints/BP_RuinBotGameinstance.DoorID` (`self.DoorID`) _asbp_ruin_bot_gameinstance)
        (`GameplayStatics.OpenLevel` (`self.LevelName`) false)))))

(fn `UserConstructionScript`
  (`BoxComponent.SetBoxExtent` (`self.Box`) (`self.LocationExtent`) false))