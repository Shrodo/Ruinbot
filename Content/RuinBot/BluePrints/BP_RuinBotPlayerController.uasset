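; Player controller for RuinBot that handles pause, sonar input and the weapon and gadget selection wheels, driving the cached character and HUD.
; Holding a wheel input freezes time via global dilation and disables aim, provided an upgrade in that category is owned and no other wheel is open.
; WheelSelection routes choices to the character's setters through a MultiGate indexed by wheel type.
; SkipUpg calls CompareUpgrade with UpgradeAll and teleports the character.
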(event `InputAction|Start` :paused true
  (params (Key :type "Key Structure"))
  (:`Pressed`
    (`self.Pause/Unpause`)))

(event `SkipUpg`
  (bind _rb_character (`self.RB_Character`))
  (`/Game/RuinBot/Character/RuinBotTestChar.CompareUpgrade` _rb_character true "NewEnumerator0")
  (`self.K2_SetActorLocation` _rb_character (49900.0 0.0 210.0) false true))

(event `Pause/Unpause`
  (bind _rb_hud (`self.RB_HUD`))
  (bind _startmenu (`/Game/RuinBot/BluePrints/HUD/BP_RuinBotHUD.StartMenu` _rb_hud))
  (`/Engine/EditorBlueprintResources/StandardMacros.FlipFlop`
    (:`A`
      (`GameplayStatics.SetGamePaused` true)
      (`/Game/RuinBot/BluePrints/HUD/BP_RuinBotHUD.PauseMenu` _rb_hud _startmenu))
    (:`B`
      (`GameplayStatics.SetGamePaused` false)
      (`/Game/RuinBot/BluePrints/HUD/BP_RuinBotHUD.Unpause` _rb_hud _startmenu))))

(event `InputAction|Sonar` :paused true
  (params (Key :type "Key Structure"))
  (:`Pressed`
    (if (`GameplayStatics.IsGamePaused`)
      (`/Game/RuinBot/BluePrints/HUD/BP_RuinBotHUD.Cancel` (`self.RB_HUD`))
      (else
        (`/Game/RuinBot/Character/RuinBotTestChar.SonarUse` (`self.RB_Character`))))))

(event `ExitIntMenu`
  (params (WidgetObj :type "UserWidget Object Reference"))
  (`/Game/RuinBot/BluePrints/HUD/BP_RuinBotHUD.ExitInteractionMenu` (`self.RB_HUD`) WidgetObj))

(event `self.ReceiveBeginPlay`
  (bind _asbp_ruin_bot_hud (cast `/Game/RuinBot/BluePrints/HUD/BP_RuinBotHUD` (`self.GetHUD`)))
  (set `self.RB_HUD` _asbp_ruin_bot_hud)
  (bind _asruin_bot_test_char (cast `/Game/RuinBot/Character/RuinBotTestChar` (`GameplayStatics.GetPlayerCharacter` 0)))
  (set `self.RB_Character` _asruin_bot_test_char))

(event `InputAction|PrimaryWheel`
  (params (Key :type "Key Structure"))
  (bind _rb_character (`self.RB_Character`))
  (bind _rb_character_2 (`self.RB_Character`))
  (bind _rb_hud (`self.RB_HUD`))
  (bind _array (`|MakeArray` (`/Game/RuinBot/Character/RuinBotTestChar.UP_Laser1` _rb_character) false false (`/Game/RuinBot/Character/RuinBotTestChar.UP_Laser2` _rb_character) false false false false))
  ;[1 1 1] SelectionWheels
  (:`Pressed`
    (if (and (`KismetArrayLibrary.Array_Contains` _array true) (not (`self.SecWheelOn`)) (not (`self.GadgetWheelOn`)))
      (set `self.PrimWheelOn` true)
      (`GameplayStatics.SetGlobalTimeDilation` 0.0)
      (`/Game/RuinBot/BluePrints/HUD/BP_RuinBotHUD.PrimWheelScreen` _rb_hud _array (`/Game/RuinBot/Character/RuinBotTestChar.PrimWeaponInt` _rb_character))
      (set `/Game/RuinBot/Character/RuinBotTestChar.AimEnabled?` false _rb_character_2)))
  (:`Released`
    (if (`self.PrimWheelOn`)
      (`GameplayStatics.SetGlobalTimeDilation` 1.0)
      (`/Game/RuinBot/BluePrints/HUD/BP_RuinBotHUD.CloseWheel` _rb_hud (`/Game/RuinBot/BluePrints/HUD/BP_RuinBotHUD.PrimWheelWJT` _rb_hud))
      (set `/Game/RuinBot/Character/RuinBotTestChar.AimEnabled?` true _rb_character_2)
      (set `self.PrimWheelOn` false))))

(event `InputAction|SecondaryWheel`
  (params (Key :type "Key Structure"))
  (bind _rb_character (`self.RB_Character`))
  (bind _rb_character_2 (`self.RB_Character`))
  (bind _rb_hud (`self.RB_HUD`))
  (bind _array (`|MakeArray` (`/Game/RuinBot/Character/RuinBotTestChar.UP_Missile` _rb_character) false false (`/Game/RuinBot/Character/RuinBotTestChar.UP_Flamethrower` _rb_character) (`/Game/RuinBot/Character/RuinBotTestChar.UP_CryoTorch` _rb_character) false false false))
  ;[1 1 1] SelectionWheels
  (:`Pressed`
    (if (and (`KismetArrayLibrary.Array_Contains` _array true) (not (`self.PrimWheelOn`)) (not (`self.GadgetWheelOn`)))
      (set `self.SecWheelOn` true)
      (`GameplayStatics.SetGlobalTimeDilation` 0.0)
      (`/Game/RuinBot/BluePrints/HUD/BP_RuinBotHUD.SecWheelScreen` _rb_hud _array (`/Game/RuinBot/Character/RuinBotTestChar.SecWeaponInt` _rb_character))
      (set `/Game/RuinBot/Character/RuinBotTestChar.AimEnabled?` false _rb_character_2)))
  (:`Released`
    (if (`self.SecWheelOn`)
      (`GameplayStatics.SetGlobalTimeDilation` 1.0)
      (`/Game/RuinBot/BluePrints/HUD/BP_RuinBotHUD.CloseWheel` _rb_hud (`/Game/RuinBot/BluePrints/HUD/BP_RuinBotHUD.SecWheelWJT` _rb_hud))
      (set `/Game/RuinBot/Character/RuinBotTestChar.AimEnabled?` true _rb_character_2)
      (set `self.SecWheelOn` false))))

(event `InputAction|GadgetWheel`
  (params (Key :type "Key Structure"))
  (bind _rb_character (`self.RB_Character`))
  (bind _rb_character_2 (`self.RB_Character`))
  (bind _rb_hud (`self.RB_HUD`))
  (bind _array (`|MakeArray` (`/Game/RuinBot/Character/RuinBotTestChar.UP_Magnet` _rb_character) false false (`/Game/RuinBot/Character/RuinBotTestChar.UP_CanCar` _rb_character) (`/Game/RuinBot/Character/RuinBotTestChar.UP_Drone` _rb_character) false false false))
  ;[1 1 1] SelectionWheels
  (:`Pressed`
    (if (and (`KismetArrayLibrary.Array_Contains` _array true) (not (`self.SecWheelOn`)) (not (`self.PrimWheelOn`)))
      (set `self.GadgetWheelOn` true)
      (`GameplayStatics.SetGlobalTimeDilation` 0.0)
      (`/Game/RuinBot/BluePrints/HUD/BP_RuinBotHUD.GadgetWheelScreen` _rb_hud _array (`/Game/RuinBot/Character/RuinBotTestChar.GadgetInt` _rb_character) (`/Game/RuinBot/Character/RuinBotTestChar.GadgetLock` (`self.RB_Character`)))
      (set `/Game/RuinBot/Character/RuinBotTestChar.AimEnabled?` false _rb_character_2)))
  (:`Released`
    (if (`self.GadgetWheelOn`)
      (`GameplayStatics.SetGlobalTimeDilation` 1.0)
      (`/Game/RuinBot/BluePrints/HUD/BP_RuinBotHUD.CloseWheel` _rb_hud (`/Game/RuinBot/BluePrints/HUD/BP_RuinBotHUD.GadgetWheelWJT` _rb_hud))
      (set `/Game/RuinBot/Character/RuinBotTestChar.AimEnabled?` true _rb_character_2)
      (set `self.GadgetWheelOn` false))))

(event `WheelSelection`
  (params (WheelType :type Integer) (Selection :type Integer))
  (bind _rb_character (`self.RB_Character`))
  ;[1 1 1] SelectionWheels
  (`|MultiGate` false false WheelType :!label _label
    (:`Out 0`
      (`/Game/RuinBot/Character/RuinBotTestChar.SetPrimaryWeapon` _rb_character Selection)
      (goto _label :!via `Reset`))
    (:`Out 1`
      (`/Game/RuinBot/Character/RuinBotTestChar.SetSecondaryWeapon` _rb_character Selection)
      (goto _label :!via `Reset`))
    (:`Out 2`
      (`/Game/RuinBot/Character/RuinBotTestChar.SetGadget` _rb_character Selection)
      (goto _label :!via `Reset`))))

(fn `UserConstructionScript`)