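; BP_Door is a sliding door that opens upward and closes through its DoorOpen and DoorClose events.
; The construction script stores the mesh's relative location as the closed position.
; DoorOpen plays a timeline whose height curve, scaled by DoorOpenDist, offsets the mesh on Z from that position, and DoorClose reverses the same timeline.
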(event `DoorOpen`
  (bind (_direction _doorheightanim) (`Timeline|Timeline_0` :!label _label)
    (:`Update`
      (`SceneComponent.K2_SetRelativeLocation` (`self.StaticMeshComponent`) (`KismetMathLibrary.MakeVector` (.x (`self.ClosedLocation`)) (.y (`self.ClosedLocation`)) (+ (.z (`self.ClosedLocation`)) (* _doorheightanim (`self.DoorOpenDist`)))) false false))))

(event `DoorClose`
  (goto _label :!via `Reverse`))

(fn `UserConstructionScript`
  (set `self.ClosedLocation` (`SceneComponent.RelativeLocation` (`self.StaticMeshComponent`))))