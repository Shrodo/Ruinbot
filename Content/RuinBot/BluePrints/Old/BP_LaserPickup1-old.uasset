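; BP_LaserPickup1-old is an older laser pickup actor for RuinBot that displays a continuously spinning LaserPack.
; Tick adds per-axis speeds to a stored rotation, wrapping each axis at ±360, and applies it in world space.
; BeginPlay caches the rotation and RuinBot HUD.
; Sonar-wave detection and Unnotice are empty: the HUD notice, custom-depth highlight, sound and notice-removal logic are disconnected, and no collection logic exists.
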(event `self.ReceiveBeginPlay`
  (set `self.CurRot` (`SceneComponent.K2_GetComponentRotation` (`self.LaserPack`)))
  (bind _asbp_ruin_bot_hud (cast `/Game/RuinBot/BluePrints/HUD/BP_RuinBotHUD` (`PlayerController.GetHUD` (`GameplayStatics.GetPlayerController` 0)))))

(event `self.PickupVolume.OnComponentBeginOverlap`
  (params (OverlappedComponent :type "PrimitiveComponent Object Reference") (OtherActor :type "Actor Object Reference") (OtherComp :type "PrimitiveComponent Object Reference") (OtherBodyIndex :type Integer) (bFromSweep :type Boolean) (SweepResult :type "HitResult Structure (by ref)"))
  (if (and (== (`GameplayStatics.GetObjectClass` OtherActor) "/Game/RuinBot/BluePrints/BP_sonarwave.BP_sonarwave_C") (not (`self.Found?`)))
    _))

(event `Unnotice`)

(event `self.ReceiveTick`
  (params (DeltaSeconds :type "Float (single-precision)"))
  (bind _returnvalue (+ (.roll (`self.CurRot`)) (`self.XRotSpeed`)))
  (bind _returnvalue_2 (+ (.yaw (`self.CurRot`)) (`self.ZRotSpeed`)))
  (bind _returnvalue_3 (+ (.pitch (`self.CurRot`)) (`self.YRotSpeed`)))
  (bind _output_get (set `self.CurRot` (`KismetMathLibrary.MakeRotator` (select `bool` (> _returnvalue 360.0) :`false` (select `bool` (< _returnvalue -360.0) :`false` _returnvalue :`true` (+ _returnvalue 360.0)) :`true` (- _returnvalue 360.0)) (select `bool` (> _returnvalue_3 360.0) :`false` (select `bool` (< _returnvalue_3 -360.0) :`false` _returnvalue_3 :`true` (+ _returnvalue_3 360.0)) :`true` (- _returnvalue_3 360.0)) (select `bool` (> _returnvalue_2 360.0) :`false` (select `bool` (< _returnvalue_2 -360.0) :`false` _returnvalue_2 :`true` (+ _returnvalue_2 360.0)) :`true` (- _returnvalue_2 360.0)))))
  (`SceneComponent.K2_SetWorldRotation` (`self.LaserPack`) _output_get false false))

(fn `UserConstructionScript`)