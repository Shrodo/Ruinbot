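; An older head pickup Blueprint for RuinBot, built to react when a sonar wave overlaps its pickup volume.
; It caches the RuinBot HUD on BeginPlay and checks the overlapping actor's class and the Found flag, but both the overlap and Unnotice lead nowhere.
; Disconnected logic would show or remove a HUD notice, highlight the head via custom depth, play a sonar sound and reset Found on a timer.
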(event `self.ReceiveBeginPlay`
  (bind _asbp_ruin_bot_hud (cast `/Game/RuinBot/BluePrints/HUD/BP_RuinBotHUD` (`PlayerController.GetHUD` (`GameplayStatics.GetPlayerController` 0)))))

(event `self.PickupVolume.OnComponentBeginOverlap`
  (params (OverlappedComponent :type "PrimitiveComponent Object Reference") (OtherActor :type "Actor Object Reference") (OtherComp :type "PrimitiveComponent Object Reference") (OtherBodyIndex :type Integer) (bFromSweep :type Boolean) (SweepResult :type "HitResult Structure (by ref)"))
  (if (and (== (`GameplayStatics.GetObjectClass` OtherActor) "/Game/RuinBot/BluePrints/BP_sonarwave.BP_sonarwave_C") (not (`self.Found?`)))
    _))

(event `Unfind`
  (set `self.Found?` false))

(event `Unnotice`)

(fn `UserConstructionScript`)