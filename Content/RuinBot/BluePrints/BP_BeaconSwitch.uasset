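; Beacon switch actor that turns on when hit by a laser projectile whose damage type matches its beacon type.
; A hit recolors its dynamic material, clears any HUD notice and starts a timer that switches it back off.
; Unconnected sonar-wave detection logic would add a HUD notice, play a ping and enable custom depth.
; The overlap event is empty, so that detection never runs.
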(event OnComponentBeginOverlap(Beacon_Mesh)
  (params (OverlappedComponent :type Primitive%20Component%20Object%20Reference) (OtherActor :type Actor%20Object%20Reference) (OtherComp :type Primitive%20Component%20Object%20Reference) (OtherBodyIndex :type Integer) (bFromSweep :type Boolean) (SweepResult :type Hit%20Result%20Structure%20%28by%20ref%29)))

(event Custom|TurnOff
  (Variables|Default|SetOn? false)
  (Rendering|Material|SetVectorParameterValueonMaterials (Variables|Default|GetBeacon_Mesh) "Color" (Math|Conversions|ToVector(LinearColor) (Variables|Default|GetBeaconInctiveColor))))

(event Custom|Unfind
  (Variables|Default|SetFound? false))

(event EventBeginPlay
  (bind _asbp_ruin_bot_hud (Utilities|Casting|CastToBP_RuinBotHUD (HUD|GetHUD (Game|GetPlayerController 0))))
  (Variables|Default|SetHUD _asbp_ruin_bot_hud))

(event Game|Damage|EventAnyDamage
  (params (Damage :type Float%20%28single-precision%29) (DamageType :type Damage%20Type%20Object%20Reference) (InstigatedBy :type Controller%20Object%20Reference) (DamageCauser :type Actor%20Object%20Reference))
  (bind _asprojectile_laser (Utilities|Casting|CastToProjectile_Laser DamageCauser))
  (if (Utilities|Enum|Equal(Enum) (Variables|/Game/RuinBot/BluePrints/Projectiles/Projectile_Laser.Projectile_Laser_C|GetDamageType _asprojectile_laser) (Variables|Default|GetBeaconType))
    (Rendering|Material|SetVectorParameterValueonMaterials (Variables|Default|GetBeacon_Mesh) "Color" (Math|Conversions|ToVector(LinearColor) (Variables|Default|GetBeaconActiveColor)))
    (Variables|Default|SetOn? true)
    (Utilities|Time|SetTimerbyEvent (delegate Custom|TurnOff) (Variables|Default|GetActivationTime))
    (Utilities|IsValid (stale _result)
      (:Is%20Valid
        (Default|DestroyWidgetObj (Variables|Default|GetHUD) (stale _result))))))

(fn ConstructionScript
  (Rendering|Material|CreateDynamicMaterialInstance (Variables|Default|GetBeacon_Mesh) 0 "/Game/RuinBot/TexMat/M_Beacon.M_Beacon" "None" :!class /Script/Engine.PrimitiveComponent)
  (CallFunction|TurnOff))