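; RuinBot game instance that applies player settings and holds the list of collected upgrade types.
; Events set SFX volume through a sound mix class override and pass resolution, window mode and VSync to GameUserSettings, committed by ApplySettings.
; Bloom toggles through a console command, and AddUpgrade adds each type only once.
; MusicBegin is empty; the persistent music startup and an older console-based resolution change are disconnected.
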(event `UpdateGameVolume`
  (params (NewVolume :type "Float (double-precision)"))
  (bind _output_get (set `self.GameVolume` NewVolume))
  (`GameplayStatics.SetSoundMixClassOverride` "/Game/RuinBot/BluePrints/RuinBotSoundMix.RuinBotSoundMix" "/Game/RuinBot/Audio/SFX.SFX" _output_get 1.0 0.0))

(event `UpdateRes/FS`
  (params (Res :type "IntPoint Structure"))
  (bind _returnvalue (`GameUserSettings.GetGameUserSettings`))
  (`GameUserSettings.SetScreenResolution` _returnvalue Res))

(event `UpdateFullscreen`
  (params (FullScreen :type Integer))
  (bind _returnvalue (`GameUserSettings.GetGameUserSettings`))
  (`GameUserSettings.SetFullscreenMode` _returnvalue (select `int` FullScreen :`0` "Windowed" :`1` "WindowedFullscreen" :`2` "Fullscreen" :!type "EWindowMode Enum")))

(event `UpdateVSync`
  (params (`VSync?` :type Boolean))
  (bind _returnvalue (`GameUserSettings.GetGameUserSettings`))
  (`GameUserSettings.SetVSyncEnabled` _returnvalue `VSync?`))

(event `UpdateBloom`
  (params (`Bloom?` :type Boolean))
  (`KismetSystemLibrary.ExecuteConsoleCommand` (`KismetStringLibrary.Concat_StrStr` "r.BloomQuality " (select `bool` `Bloom?` :`false` "0" :`true` "1")) (`GameplayStatics.GetPlayerController` 0)))

(event `ApplySettings`
  (bind _returnvalue (`GameUserSettings.GetGameUserSettings`))
  (`GameUserSettings.ApplySettings` _returnvalue true))

(event `AddUpgrade`
  (params (Type :type "/Game/RuinBot/BluePrints/UpgradeType Enum" :default "NewEnumerator0"))
  (`KismetArrayLibrary.Array_AddUnique` (`self.Upgrades`) Type))

(event `MusicBegin`)