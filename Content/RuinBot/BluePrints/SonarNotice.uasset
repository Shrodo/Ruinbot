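; SonarNotice is a component that reveals its owning actor when a sonar wave overlaps it.
; On a BP_sonarwave hit, it requests a notice widget from BP_RuinBotHUD, enables custom-depth stencil rendering on the mesh and plays a pitch-varied sonar sound.
; A Found flag blocks retriggers until a timer clears it and destroys the widget, while custom depth stays enabled.
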(event `self.ReceiveBeginPlay`
  (`|ExecutionSequence`
    (:`then_0`
      (bind _asbp_ruin_bot_hud (cast `/Game/RuinBot/BluePrints/HUD/BP_RuinBotHUD` (`PlayerController.GetHUD` (`GameplayStatics.GetPlayerController` 0)))))
    (:`then_1`
      (set `self.Mesh` (`|GetArrayItem` (`Actor.K2_GetComponentsByClass` (`self.GetOwner`) "/Script/Engine.PrimitiveComponent") (`self.MeshIndex`))))))

(event `Overlap`
  (params (OtherActor :type "Actor Object Reference") (Mesh :type "PrimitiveComponent Object Reference"))
  (bind _mesh (`self.Mesh`))
  (if (and (== (`GameplayStatics.GetObjectClass` OtherActor) "/Game/RuinBot/BluePrints/BP_sonarwave.BP_sonarwave_C") (not (`self.Found?`)))
    (bind _result (`/Game/RuinBot/BluePrints/HUD/BP_RuinBotHUD.Notice Object` (stale `self.ReceiveBeginPlay` _asbp_ruin_bot_hud) (`self.GetOwner`) (`self.NoticeColor`) (0.0 0.0) (`self.NoticeOffset`) (`GameplayStatics.GetPlayerController` 0) (`self.NoticeDuration`) null null (`self.NoticeDescription`)))
    (`/Engine/EditorBlueprintResources/StandardMacros.IsValid` _mesh
      (:`Is Valid`
        (`PrimitiveComponent.SetRenderCustomDepth` _mesh true)
        (`PrimitiveComponent.SetCustomDepthStencilValue` _mesh (`self.DepthStencil`)))
      (:`Is Not Valid`
        _))
    (`GameplayStatics.PlaySoundAtLocation` "/Game/RuinBot/Audio/Sonar4.Sonar4" (`SceneComponent.K2_GetComponentLocation` (`Actor.RootComponent` (`self.GetOwner`))) (struct) 2.0 (`KismetMathLibrary.RandomFloatInRange` 0.95 1.05) 0.0 null null null)
    (set `self.Found?` true)
    (`KismetSystemLibrary.K2_SetTimerDelegate` (delegate `Unfind`) (`self.NoticeDuration`))))

(event `Unfind`
  (set `self.Found?` false)
  (`self.Unnotice`))

(event `Unnotice`
  (`/Game/RuinBot/BluePrints/HUD/BP_RuinBotHUD.DestroyWidgetObj` (stale `self.ReceiveBeginPlay` _asbp_ruin_bot_hud) (stale `Overlap` _result)))