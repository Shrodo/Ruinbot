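; RB_Gamemode is a RuinBot game mode that decides where the player spawns based on a door ID.
; Its ChoosePlayerStart override reads DoorID from BP_RuinBotGameinstance and returns the PlayerStart whose tag matches, falling back to the first one found.
; BeginPlay is empty, and a leftover console command node is never run.
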(event `self.ReceiveBeginPlay`)

(fn `ChoosePlayerStart`
  (params (Player :type "Controller Object Reference"))
  (returns (ReturnValue :type "Actor Object Reference"))
  (bind _asbp_ruin_bot_gameinstance (cast `/Game/RuinBot/BluePrints/BP_RuinBotGameinstance` (`GameplayStatics.GetGameInstance`)))
  (bind _outactors (`GameplayStatics.GetAllActorsOfClass` "/Script/Engine.PlayerStart"))
  (for _array_element _outactors
    (if (== (`PlayerStart.PlayerStartTag` _array_element) (`/Game/RuinBot/BluePrints/BP_RuinBotGameinstance.DoorID` _asbp_ruin_bot_gameinstance))
      (return _array_element)))
  (return (`|GetArrayItem` _outactors)))

(fn `UserConstructionScript`)