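; Master upgrade pickup for RuinBot that is revealed when a sonar wave overlaps its pickup volume.
; On detection it shows a HUD notice, enables custom depth on its mesh and plays a randomly pitched ping.
; A timer then clears the found flag and removes the notice, allowing re-detection, while custom depth stays on.
; The graph holds no collection or upgrade logic.
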(event `self.ReceiveBeginPlay`
  (bind _asbp_ruin_bot_hud (cast `/Game/RuinBot/BluePrints/HUD/BP_RuinBotHUD` (`PlayerController.GetHUD` (`GameplayStatics.GetPlayerController` 0)))))

(event `self.PickupVolume.OnComponentBeginOverlap`
  (params (OverlappedComponent :type "PrimitiveComponent Object Reference") (OtherActor :type "Actor Object Reference") (OtherComp :type "PrimitiveComponent Object Reference") (OtherBodyIndex :type Integer) (bFromSweep :type Boolean) (SweepResult :type "HitResult Structure (by ref)"))
  (if (and (== (`GameplayStatics.GetObjectClass` OtherActor) "/Game/RuinBot/BluePrints/BP_sonarwave.BP_sonarwave_C") (not (`self.Found?`)))
    (bind _result (`/Game/RuinBot/BluePrints/HUD/BP_RuinBotHUD.Notice Object` (stale `self.ReceiveBeginPlay` _asbp_ruin_bot_hud) self (`self.NoticeColor`) (0.0 0.0) (`self.NoticeOffset`) (`GameplayStatics.GetPlayerController` 0) (`self.NoticeDuration`) null null (`self.NoticeDescription`)))
    (bind _staticmesh (`self.StaticMesh`)
      (:`then`
        (`PrimitiveComponent.SetRenderCustomDepth` _staticmesh true))
      (:`else`
        _))
    (`GameplayStatics.PlaySoundAtLocation` "/Game/RuinBot/Audio/Sonar4.Sonar4" (`SceneComponent.K2_GetComponentLocation` (`self.PickupVolume`)) (struct) 2.0 (`KismetMathLibrary.RandomFloatInRange` 0.95 1.05) 0.0 null null null)
    (set `self.Found?` true)
    (`KismetSystemLibrary.K2_SetTimerDelegate` (delegate `Unfind`) (`self.NoticeDuration`))))

(event `Unfind`
  (set `self.Found?` false)
  (`self.Unnotice`))

(event `Unnotice`
  (`/Game/RuinBot/BluePrints/HUD/BP_RuinBotHUD.DestroyWidgetObj` (stale `self.ReceiveBeginPlay` _asbp_ruin_bot_hud) (stale `self.PickupVolume.OnComponentBeginOverlap` _result)))

(fn `UserConstructionScript`)