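; CliffSpline is a construction-script Blueprint that lays spline mesh sections along an editable spline, apparently to build cliffs.
; It divides the spline by SectionLength, optionally adds a remainder piece, and gives each section query-and-physics collision.
; Tangents are clamped to section length, and GapFill extends each end to cover seams.
; A Reset flag restores default points, and ClosedLoop controls looping.
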(fn `UserConstructionScript`
  (bind _spline (`self.Spline`))
  (bind _section_length (`self.Section Length`))
  (bind _section_length_2 (`self.Section Length`))
  (bind _spline_2 (`self.Spline`))
  (bind _returnvalue (`KismetMathLibrary.FTrunc` (/ (`SplineComponent.GetSplineLength` _spline) (`self.Section Length`))))
  (if (`self.Reset`)
    (for _index (range (+ (`SplineComponent.GetNumberOfSplinePoints` _spline_2) 1))
      (`SplineComponent.RemoveSplinePoint` _spline_2 _index true))
    (`SplineComponent.SetSplinePoints` (`self.Spline`) (`self.DefaultPoints`) "Local" true)
    (set `self.Reset` false))
  (`SplineComponent.SetClosedLoop` (`self.Spline`) (`self.ClosedLoop?`) true)
  (`SplineComponent.SetClosedLoop` _spline (`self.ClosedLoop?`) true)
  (for _index_2 (range (+ (select `bool` (`self.AddRemainder?`) :`false` (- _returnvalue 1) :`true` _returnvalue) 1))
    (bind _returnvalue_2 (`AddComponent|NODE_AddSplineMeshComponent-0`))
    (`PrimitiveComponent.SetCollisionEnabled` _returnvalue_2 "QueryAndPhysics")
    (bind _returnvalue_3 (* _index_2 _section_length_2))
    (bind _returnvalue_4 (+ (* (+ _index_2 1) _section_length_2) (`self.GapFill`)))
    (`SplineMeshComponent.SetStartAndEnd` _returnvalue_2 (`SplineComponent.GetLocationAtDistanceAlongSpline` _spline _returnvalue_3 "Local") (`KismetMathLibrary.ClampVectorSize` (`SplineComponent.GetTangentAtDistanceAlongSpline` _spline _returnvalue_3 "Local") 0.0 _section_length) (`SplineComponent.GetLocationAtDistanceAlongSpline` _spline _returnvalue_4 "Local") (`KismetMathLibrary.ClampVectorSize` (`SplineComponent.GetTangentAtDistanceAlongSpline` _spline _returnvalue_4 "Local") 0.0 _section_length) true)))