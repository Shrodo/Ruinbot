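; BP_Bird is an ambient bird that flees and vanishes when a space pirate character or NPC enters its Detect volume.
; On overlap it reorients, plays a sound and sets a target point directly away from the intruder, scaled by their separation.
; Tick interpolates it there, using horizontal progress to sample curves for arc height and material transparency.
; The actor destroys itself near the end of the flight.
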(event `self.Detect.OnComponentBeginOverlap`
  (params (OverlappedComponent :type "PrimitiveComponent Object Reference") (OtherActor :type "Actor Object Reference") (OtherComp :type "PrimitiveComponent Object Reference") (OtherBodyIndex :type Integer) (bFromSweep :type Boolean) (SweepResult :type "HitResult Structure (by ref)"))
  (bind _returnvalue (`GameplayStatics.GetObjectClass` OtherActor))
  (if (or (== _returnvalue "/Game/Spirate/Characters/BP_SpacePirateChar.BP_SpacePirateChar_C") (== _returnvalue "/Game/AI/NPC_Char.NPC_Char_C"))
    (`self.MakeFlyAwayPoint` OtherActor)))

(event `MakeFlyAwayPoint`
  (params (AwayFrom :type "Actor Object Reference"))
  (bind _returnvalue (`SceneComponent.K2_GetComponentLocation` (`self.CapsuleComponent`)))
  (bind _returnvalue_2 (* (- (`self.K2_GetActorLocation` AwayFrom) _returnvalue) 3.0))
  (bind _returnvalue_3 (- _returnvalue _returnvalue_2))
  (set `self.CurPos` _returnvalue)
  (`SceneComponent.K2_SetWorldRotation` (`self.CapsuleComponent`) (`KismetMathLibrary.ComposeRotators` (`KismetMathLibrary.Conv_VectorToRotator` _returnvalue_2) (struct :`Yaw` 180.0)) false false)
  (`GameplayStatics.PlaySoundAtLocation` "/Game/RuinBot/Audio/BirdFly.BirdFly" _returnvalue (struct) 1.0 1.0 0.0 null null null)
  (`self.FlyToPoint` _returnvalue_3 (`KismetMathLibrary.VSize` (- _returnvalue _returnvalue_3)) _returnvalue))

(event `FlyToPoint`
  (params (FlyTo :type "Vector Structure") (InitDist :type "Float (double-precision)") (InitPos :type "Vector Structure"))
  (set `self.FlyActive?` (not (> (- 1.0 (/ (`KismetMathLibrary.VSize` (- (`KismetMathLibrary.MakeVector` (.x (`self.CurPos`)) (.y (`self.CurPos`))) (`KismetMathLibrary.MakeVector` (.x FlyTo) (.y FlyTo)))) InitDist)) 0.9))))

(event `self.ReceiveTick`
  (params (DeltaSeconds :type "Float (single-precision)"))
  (if (`self.FlyActive?`)
    (bind _x (.x (stale `FlyToPoint` FlyTo)))
    (bind _y (.y (stale `FlyToPoint` FlyTo)))
    (bind _returnvalue (/ (`KismetMathLibrary.VSize` (- (`KismetMathLibrary.MakeVector` (.x (`self.CurPos`)) (.y (`self.CurPos`))) (`KismetMathLibrary.MakeVector` _x _y))) (stale `FlyToPoint` InitDist)))
    (bind _returnvalue_2 (- 1.0 _returnvalue))
    (if (> _returnvalue_2 0.9)
      (`/Engine/EditorBlueprintResources/StandardMacros.IsValid` self
        (:`Is Valid`
          (`self.K2_DestroyActor`)))
      (else
        (`MeshComponent.SetScalarParameterValueOnMaterials` (`self.Mesh`) "transparency" (`CurveFloat.GetFloatValue` (`self.VisCurve`) _returnvalue_2))
        (bind _output_get (set `self.CurPos` (`KismetMathLibrary.VInterpTo` (`self.CurPos`) (`KismetMathLibrary.MakeVector` _x _y (+ (* (`CurveFloat.GetFloatValue` (`self.FlyCurve`) _returnvalue_2) (`self.FlyHeight`)) (`KismetMathLibrary.Lerp` (.z (stale `FlyToPoint` InitPos)) (.z (stale `FlyToPoint` FlyTo)) _returnvalue))) DeltaSeconds (`self.FlySpeed`))))
        (`SceneComponent.K2_SetWorldLocation` (`self.CapsuleComponent`) _output_get false false)))))

(event `self.ReceiveBeginPlay`
  (`PrimitiveComponent.CreateDynamicMaterialInstance` (`self.Mesh`) 0 "/Game/RuinBot/TexMat/M_Bird1.M_Bird1" "None"))

(fn `UserConstructionScript`)