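; BP_BirdSpawn is a spawner actor that keeps at most one ambient BP_Bird alive around its SpawnPoint.
; A looping timer, with an interval randomized once at BeginPlay, calls SpawnBird.
; SpawnBird only acts when the player is far from the SpawnPoint and the tracked bird is invalid.
; It then spawns a new bird at a random navigable point within a radius of SpawnPoint and stores it.
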(event `self.ReceiveBeginPlay`
  (`KismetSystemLibrary.K2_SetTimer` null "SpawnBird" (`KismetMathLibrary.RandomFloatInRange` 20.0 200.0) true))

(event `SpawnBird`
  (bind _returnvalue (`SceneComponent.K2_GetComponentLocation` (`self.SpawnPoint`)))
  (if (> (`KismetMathLibrary.VSize` (- (`self.K2_GetActorLocation` (`GameplayStatics.GetPlayerCharacter` 0)) _returnvalue)) 3000.0)
    (`/Engine/EditorBlueprintResources/StandardMacros.IsValid` (`self.OurBird`)
      (:`Is Not Valid`
        (bind _returnvalue_2 (`|SpawnActorFromClass` "/Game/RuinBot/BluePrints/BP_Bird.BP_Bird_C" (`KismetMathLibrary.MakeTransform` (`NavigationSystem.GetRandomPointInNavigableRadius` _returnvalue 3000.0) (`KismetMathLibrary.MakeRotator` 0.0 0.0 (`KismetMathLibrary.RandomFloat`))) "Undefined" "OverrideRootScale"))
        (set `self.OurBird` _returnvalue_2)))))

(fn `UserConstructionScript`)