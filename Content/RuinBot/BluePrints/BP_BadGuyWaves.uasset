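; BP_BadGuyWaves is a wave manager that runs a timed countdown loop for escalating enemy waves.
; Each countdown increments the wave, raises the enemy count, updates the pirate character and RuinBot HUD, then schedules NewWave.
; NewWave is empty: the logic that spawns NPC_Char AI at random navigable points with HUD markers is disconnected.
; EndWave restarts the countdown, though nothing in this graph calls it.
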(event `self.ReceiveBeginPlay`
  (bind _asbp_ruin_bot_hud (cast `/Game/RuinBot/BluePrints/HUD/BP_RuinBotHUD` (`PlayerController.GetHUD` (`GameplayStatics.GetPlayerController` 0))))
  (set `self.RBHUD` _asbp_ruin_bot_hud)
  (bind _asbp_space_pirate_char (cast `/Game/Spirate/Characters/BP_SpacePirateChar` (`GameplayStatics.GetPlayerCharacter` 0)))
  (`KismetSystemLibrary.K2_SetTimer` null "WaveCountdown" 5.0))

(event `WaveCountdown`
  (bind _wave (`self.Wave`))
  (bind _output_get (set `self.Wave` (+ _wave 1)))
  (`/Game/Spirate/Characters/BP_SpacePirateChar.SetWave` (stale `self.ReceiveBeginPlay` _asbp_space_pirate_char) _output_get)
  (set `self.AmountOfBaddies` (+ (`self.AmountOfBaddies`) 2))
  (bind _returnvalue (`KismetSystemLibrary.K2_SetTimer` null "NewWave" 10.0))
  (set `self.NextWaveTimer` _returnvalue)
  (`/Game/RuinBot/BluePrints/HUD/BP_RuinBotHUD.NewWave` (`self.RBHUD`) _wave))

(event `NewWave`)

(event `EndWave`
  (`KismetSystemLibrary.K2_SetTimer` null "WaveCountdown" 5.0))

(fn `UserConstructionScript`)