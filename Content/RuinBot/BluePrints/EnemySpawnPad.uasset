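; EnemySpawnPad is a spawn pad Blueprint that creates groups of regular and sniper NPC enemies around itself.
; Spawn takes a count for each type and calls SpawnType, which places each NPC at a random reachable navmesh point within a fixed radius, with random yaw.
; Each type receives its own laser projectile class.
; The UserVolume overlap event is empty, and the SonarNotice overlap logic is disconnected.
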(event `SpawnType`
  (params (Num :type Integer) (Class :type "Actor Class Reference"))
  (bind _returnvalue (`KismetMathLibrary.MakeTransform` (`NavigationSystemV1.K2_GetRandomReachablePointInRadius` (`SceneComponent.K2_GetComponentLocation` (`self.DefaultSceneRoot`)) 2500.0 null null) (`KismetMathLibrary.MakeRotator` 0.0 0.0 (`KismetMathLibrary.RandomFloatInRange` 0.0 360.0))))
  (for _ (range Num)
    (if (== Class "/Game/RuinBot/AI/NPC_SniperChar.NPC_SniperChar_C")
      (`|SpawnActorFromClass` "/Game/RuinBot/AI/NPC_SniperChar.NPC_SniperChar_C" _returnvalue "Undefined" "OverrideRootScale" null "NewEnumerator1" null "/Game/RuinBot/BluePrints/Projectiles/Projectie_SniperLaser.Projectie_SniperLaser_C" 0.7 160.0 null)
      (else
        (`|SpawnActorFromClass` "/Game/RuinBot/AI/NPC_Char.NPC_Char_C" _returnvalue "Undefined" "OverrideRootScale" null "NewEnumerator1" null "/Game/RuinBot/BluePrints/Projectiles/Projectile_Laser.Projectile_Laser_C" 0.0 160.0 null)))))

(event `Spawn`
  (params (DefNum :type Integer) (SnipNum :type Integer))
  (`self.SpawnType` DefNum "/Game/RuinBot/AI/NPC_Char.NPC_Char_C")
  (`self.SpawnType` SnipNum "/Game/RuinBot/AI/NPC_SniperChar.NPC_SniperChar_C"))

(event `self.UserVolume.OnComponentBeginOverlap`
  (params (OverlappedComponent :type "PrimitiveComponent Object Reference") (OtherActor :type "Actor Object Reference") (OtherComp :type "PrimitiveComponent Object Reference") (OtherBodyIndex :type Integer) (bFromSweep :type Boolean) (SweepResult :type "HitResult Structure (by ref)")))

(fn `UserConstructionScript`)