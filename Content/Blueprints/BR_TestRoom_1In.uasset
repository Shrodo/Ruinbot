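; BR_TestRoom_1In is a test room Blueprint whose rock and ground meshes take on the current planet's colors.
; On BeginPlay it creates one dynamic instance of M_Zrock shared by the rock meshes and one of Ground1 for a single mesh.
; It reads PlanetPrimary and PlanetSecondary from BP_SpaceController, tinting the rocks with both and the ground with only the secondary.
; Nothing is applied if the player controller cast fails.
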(event `self.ReceiveBeginPlay`
  (bind _asbp_space_controller (cast `/Game/Blueprints/BP_SpaceController` (`GameplayStatics.GetPlayerController` 0)))
  (bind _returnvalue (`KismetMaterialLibrary.CreateDynamicMaterialInstance` "/Game/Materials/M_Zrock.M_Zrock"))
  (`PrimitiveComponent.SetMaterial` (`self.StaticMesh1`) 0 _returnvalue)
  (`PrimitiveComponent.SetMaterial` (`self. grgeg`) 0 _returnvalue)
  (`PrimitiveComponent.SetMaterial` (`self.StaticMesh12`) 0 _returnvalue)
  (`PrimitiveComponent.SetMaterial` (`self.StaticMesh11`) 0 _returnvalue)
  (`PrimitiveComponent.SetMaterial` (`self.StaticMesh10`) 0 _returnvalue)
  (`PrimitiveComponent.SetMaterial` (`self.StaticMesh7`) 0 _returnvalue)
  (`PrimitiveComponent.SetMaterial` (`self.rrrrr`) 0 _returnvalue)
  (`PrimitiveComponent.SetMaterial` (`self.StaticMesh8`) 0 _returnvalue)
  (`PrimitiveComponent.SetMaterial` (`self. rrr`) 0 _returnvalue)
  (`PrimitiveComponent.SetMaterial` (`self.StaticMesh9`) 0 _returnvalue)
  (`PrimitiveComponent.SetMaterial` (`self.StaticMesh6`) 0 _returnvalue)
  (`PrimitiveComponent.SetMaterial` (`self.StaticMesh2`) 0 _returnvalue)
  (`PrimitiveComponent.SetMaterial` (`self.StaticMesh3`) 0 _returnvalue)
  (`PrimitiveComponent.SetMaterial` (`self.StaticMesh4`) 0 _returnvalue)
  (`PrimitiveComponent.SetMaterial` (`self.rocky`) 0 _returnvalue)
  (`PrimitiveComponent.SetMaterial` (`self.StaticMesh13`) 0 _returnvalue)
  (bind _returnvalue_2 (`KismetMaterialLibrary.CreateDynamicMaterialInstance` "/Game/Materials/Ground1.Ground1"))
  (`PrimitiveComponent.SetMaterial` (`self.StaticMesh5`) 0 _returnvalue_2)
  (`MaterialInstanceDynamic.SetVectorParameterValue` _returnvalue "PrimaryColor" (`KismetMathLibrary.Conv_VectorToLinearColor` (`/Game/Blueprints/BP_SpaceController.PlanetPrimary` _asbp_space_controller)))
  (bind _returnvalue_3 (`KismetMathLibrary.Conv_VectorToLinearColor` (`/Game/Blueprints/BP_SpaceController.PlanetSecondary` _asbp_space_controller)))
  (`MaterialInstanceDynamic.SetVectorParameterValue` _returnvalue "SecondaryColor" _returnvalue_3)
  (`MaterialInstanceDynamic.SetVectorParameterValue` _returnvalue_2 "SecondaryColor" _returnvalue_3))

(fn `UserConstructionScript`)