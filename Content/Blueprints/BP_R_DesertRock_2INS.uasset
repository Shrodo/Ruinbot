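; Desert rock Blueprint that tints its rock, rock pile and fog plane meshes to match the current planet's colors.
; On BeginPlay, for each SpaceCharacter found, it stores the character, creates dynamic materials and assigns them by static mesh.
; The space controller's primary and secondary colors, blended halfway toward grey, tint the rocks, while the third colors the fog.
; Tick records the stored character's closest distance and capsule relative location.
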(event `self.ReceiveBeginPlay`
  (bind _asbp_space_controller (cast `/Game/Blueprints/BP_SpaceController` (`GameplayStatics.GetPlayerController` 0)))
  (bind _outactors (`GameplayStatics.GetAllActorsOfClass` "/Game/Blueprints/SpaceCharacter.SpaceCharacter_C"))
  (for _array_element _outactors
    (set `self.Character` _array_element)
    (bind _returnvalue (`KismetMaterialLibrary.CreateDynamicMaterialInstance` "/Game/Materials/M_DesertRock1.M_DesertRock1"))
    (bind _returnvalue_2 (`KismetMaterialLibrary.CreateDynamicMaterialInstance` "/Game/Materials/M_DesertRock2.M_DesertRock2"))
    (bind _returnvalue_3 (`KismetMaterialLibrary.CreateDynamicMaterialInstance` "/Game/Materials/M_DesertRockPile.M_DesertRockPile"))
    (bind _returnvalue_4 (`KismetMaterialLibrary.CreateDynamicMaterialInstance` "/Game/Materials/M_DesertSmRock1.M_DesertSmRock1"))
    (bind _returnvalue_5 (`KismetMaterialLibrary.CreateDynamicMaterialInstance` "/Game/Materials/M_DesertSmRock2.M_DesertSmRock2"))
    (bind _returnvalue_6 (`KismetMaterialLibrary.CreateDynamicMaterialInstance` "/Game/Materials/M_FogPlane.M_FogPlane"))
    (for _array_element_2 (`self.K2_GetComponentsByClass` "/Script/Engine.StaticMeshComponent")
      (bind _asstatic_mesh_component (cast `StaticMeshComponent` _array_element_2))
      (bind _staticmesh (`StaticMeshComponent.StaticMesh` _asstatic_mesh_component))
      (if (== _staticmesh "/Game/Meshes/SM_DesertRock1.SM_DesertRock1")
        (`PrimitiveComponent.SetMaterial` _asstatic_mesh_component 0 _returnvalue)
        (elif (== _staticmesh "/Game/Meshes/SM_DesertRock2.SM_DesertRock2")
          (`PrimitiveComponent.SetMaterial` _asstatic_mesh_component 0 _returnvalue_2)
          (elif (== _staticmesh "/Game/Meshes/SM_DesertSmallRock1.SM_DesertSmallRock1")
            (`PrimitiveComponent.SetMaterial` _asstatic_mesh_component 0 _returnvalue_4)
            (elif (== _staticmesh "/Game/Meshes/SM_DesertSmallRock2.SM_DesertSmallRock2")
              (`PrimitiveComponent.SetMaterial` _asstatic_mesh_component 0 _returnvalue_5)
              (elif (== _staticmesh "/Game/Meshes/SM_RockPile1.SM_RockPile1")
                (`PrimitiveComponent.SetMaterial` _asstatic_mesh_component 0 _returnvalue_3)
                (elif (== _staticmesh "/Game/Shapes/Shape_Plane.Shape_Plane")
                  (`PrimitiveComponent.SetMaterial` _asstatic_mesh_component 0 _returnvalue_6))))))))
    (`MaterialInstanceDynamic.SetVectorParameterValue` _returnvalue "PrimaryColor" (`KismetMathLibrary.LinearColorLerp` (`KismetMathLibrary.Conv_VectorToLinearColor` (`/Game/Blueprints/BP_SpaceController.PlanetPrimary` _asbp_space_controller)) (struct :`R` 0.5 :`G` 0.5 :`B` 0.5 :`A` 1.0) 0.5))
    (`MaterialInstanceDynamic.SetVectorParameterValue` _returnvalue_2 "PrimaryColor" (`KismetMathLibrary.LinearColorLerp` (`KismetMathLibrary.Conv_VectorToLinearColor` (`/Game/Blueprints/BP_SpaceController.PlanetPrimary` _asbp_space_controller)) (struct :`R` 0.5 :`G` 0.5 :`B` 0.5 :`A` 1.0) 0.5))
    (`MaterialInstanceDynamic.SetVectorParameterValue` _returnvalue_3 "PrimaryColor" (`KismetMathLibrary.LinearColorLerp` (`KismetMathLibrary.Conv_VectorToLinearColor` (`/Game/Blueprints/BP_SpaceController.PlanetPrimary` _asbp_space_controller)) (struct :`R` 0.5 :`G` 0.5 :`B` 0.5 :`A` 1.0) 0.5))
    (`MaterialInstanceDynamic.SetVectorParameterValue` _returnvalue_4 "PrimaryColor" (`KismetMathLibrary.LinearColorLerp` (`KismetMathLibrary.Conv_VectorToLinearColor` (`/Game/Blueprints/BP_SpaceController.PlanetPrimary` _asbp_space_controller)) (struct :`R` 0.5 :`G` 0.5 :`B` 0.5 :`A` 1.0) 0.5))
    (`MaterialInstanceDynamic.SetVectorParameterValue` _returnvalue_5 "PrimaryColor" (`KismetMathLibrary.LinearColorLerp` (`KismetMathLibrary.Conv_VectorToLinearColor` (`/Game/Blueprints/BP_SpaceController.PlanetPrimary` _asbp_space_controller)) (struct :`R` 0.5 :`G` 0.5 :`B` 0.5 :`A` 1.0) 0.5))
    (`MaterialInstanceDynamic.SetVectorParameterValue` _returnvalue "SecondaryColor" (`KismetMathLibrary.LinearColorLerp` (`KismetMathLibrary.Conv_VectorToLinearColor` (`/Game/Blueprints/BP_SpaceController.PlanetSecondary` _asbp_space_controller)) (struct :`R` 0.64 :`G` 0.64 :`B` 0.64 :`A` 1.0) 0.5))
    (`MaterialInstanceDynamic.SetVectorParameterValue` _returnvalue_2 "SecondaryColor" (`KismetMathLibrary.LinearColorLerp` (`KismetMathLibrary.Conv_VectorToLinearColor` (`/Game/Blueprints/BP_SpaceController.PlanetSecondary` _asbp_space_controller)) (struct :`R` 0.64 :`G` 0.64 :`B` 0.64 :`A` 1.0) 0.5))
    (`MaterialInstanceDynamic.SetVectorParameterValue` _returnvalue_3 "SecondaryColor" (`KismetMathLibrary.LinearColorLerp` (`KismetMathLibrary.Conv_VectorToLinearColor` (`/Game/Blueprints/BP_SpaceController.PlanetSecondary` _asbp_space_controller)) (struct :`R` 0.64 :`G` 0.64 :`B` 0.64 :`A` 1.0) 0.5))
    (`MaterialInstanceDynamic.SetVectorParameterValue` _returnvalue_4 "SecondaryColor" (`KismetMathLibrary.LinearColorLerp` (`KismetMathLibrary.Conv_VectorToLinearColor` (`/Game/Blueprints/BP_SpaceController.PlanetSecondary` _asbp_space_controller)) (struct :`R` 0.64 :`G` 0.64 :`B` 0.64 :`A` 1.0) 0.5))
    (`MaterialInstanceDynamic.SetVectorParameterValue` _returnvalue_5 "SecondaryColor" (`KismetMathLibrary.LinearColorLerp` (`KismetMathLibrary.Conv_VectorToLinearColor` (`/Game/Blueprints/BP_SpaceController.PlanetSecondary` _asbp_space_controller)) (struct :`R` 0.64 :`G` 0.64 :`B` 0.64 :`A` 1.0) 0.5))
    (`MaterialInstanceDynamic.SetScalarParameterValue` _returnvalue "GradHeight" -20.0)
    (`MaterialInstanceDynamic.SetScalarParameterValue` _returnvalue_2 "GradHeight" -20.0)
    (`MaterialInstanceDynamic.SetScalarParameterValue` _returnvalue_3 "GradHeight" -20.0)
    (`MaterialInstanceDynamic.SetScalarParameterValue` _returnvalue_4 "GradHeight" -20.0)
    (`MaterialInstanceDynamic.SetScalarParameterValue` _returnvalue_5 "GradHeight" -20.0)
    (`MaterialInstanceDynamic.SetVectorParameterValue` _returnvalue_6 "FogColor" (`KismetMathLibrary.Conv_VectorToLinearColor` (`/Game/Blueprints/BP_SpaceController.PlanetThird` _asbp_space_controller)))))

(event `self.ReceiveTick`
  (params (DeltaSeconds :type "Float (single-precision)"))
  (bind _capsulecomponent (`Character.CapsuleComponent` (`self.Character`)))
  (bind _returnvalue (`KismetMathLibrary.VSize` (- (`SceneComponent.K2_GetComponentLocation` (`self.SharedRoot`)) (`SceneComponent.K2_GetComponentLocation` _capsulecomponent))))
  (if (< _returnvalue (`self.NearestDist`))
    (set `self.NearestRelLoc` (`SceneComponent.RelativeLocation` _capsulecomponent))
    (set `self.NearestDist` _returnvalue)))

(fn `UserConstructionScript`)