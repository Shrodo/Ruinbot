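; Procedurally generated planet actor that spins, orbits its owner, and passes its data to BP_SpaceController when the player overlaps it.
; Random streams seeded by galaxy seed, position and planet number derive colors, water, type, size and syllable-built name.
; Names retry against the GameInstance list up to a limit; only unique ones get built.
; Random land values draw into a small canvas render target feeding surface and UI map materials.
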(event `self.ReceiveActorBeginOverlap`
  (params (OtherActor :type "Actor Object Reference"))
  ;[0.1456 0.1823 1] Setting 'Current Planet' Colors
  (if (== (`GameplayStatics.GetObjectClass` OtherActor) "/Game/Blueprints/BP_Player.BP_Player_C")
    (bind _asbp_space_controller (cast `/Game/Blueprints/BP_SpaceController` (`GameplayStatics.GetPlayerController` 0)))
    (`/Game/Blueprints/BP_SpaceController.Set Current Planet Colors` _asbp_space_controller (`self.PrimaryColor`) (`self.SecondaryColor`) (`self.ThirdColor`) (* (`self.PlanetPos`) (`KismetMathLibrary.Conv_IntToDouble` (`self.PlanetNum`))) (`self.Type`) (`self.PlanetName`) (`self.PlanetMapUI`) (`self.MapCoords`) (`self.LandValues`) (`self.WaterCover`) (`self.SunColor`))))

(event `AttemptPlanetBuild`
  (bind _planetmapui (`self.PlanetMapUI`))
  (bind _planetmesh (`self.PlanetMesh`))
  (bind _attemptnum (`self.AttemptNum`))
  (bind _returnvalue (+ (`KismetMathLibrary.FTrunc` (+ (.x (`self.PlanetPos`)) (.y (`self.PlanetPos`)) (.z (`self.PlanetPos`)))) (`self.gSeed`) (`self.PlanetNum`)))
  (bind _returnvalue_2 (`KismetMathLibrary.RandomIntegerInRangeFromStream` 0 28 (`KismetMathLibrary.MakeRandomStream` (+ (* _returnvalue 15) 15 _attemptnum))))
  (bind _returnvalue_3 (select `int` (`KismetMathLibrary.RandomIntegerInRangeFromStream` 0 7 (`KismetMathLibrary.MakeRandomStream` (+ _returnvalue 10))) :`0` "Rocky" :`1` "Jungle" :`2` "Ice" :`3` "Lava" :`4` "Swamp" :`5` "Sand" :`6` "Temperate" :`7` "Tropical"))
  (bind _returnvalue_4 (select `int` (`KismetMathLibrary.RandomIntegerInRangeFromStream` 0 32 (`KismetMathLibrary.MakeRandomStream` (+ _returnvalue 14 _attemptnum))) :`0` "Ga" :`1` "Ge" :`2` "Ra" :`3` "Ren" :`4` "Rii" :`5` "Ae" :`6` "A" :`7` "O" :`8` "Mo" :`9` "I" :`10` "Sra" :`11` "No" :`12` "Mi" :`13` "He" :`14` "Ha" :`15` "Xu" :`16` "Zii" :`17` "Ke" :`18` "Ku" :`19` "De" :`20` "Te" :`21` "Vu" :`22` "Jai" :`23` "Qe" :`24` "Yu" :`25` "Lo" :`26` "Cri" :`27` "Sa" :`28` "Il" :`29` "Ax" :`30` "Tre" :`31` "Vai" :`32` "Zra"))
  (bind _returnvalue_5 (select `int` _returnvalue_2 :`0` "no" :`1` "baan" :`2` "mu" :`3` "bis" :`4` "ten" :`5` "ris" :`6` "gand" :`7` "be" :`8` "to" :`9` "kuu" :`10` "in" :`11` "ho" :`12` "yu" :`13` "wen" :`14` "ju" :`15` "ken" :`16` "go" :`17` "ta" :`18` "mar" :`19` "bo" :`20` "rad" :`21` "ven" :`22` "fre" :`23` "shi" :`24` "sen" :`25` "la" :`26` "wi" :`27` "'bi" :`28` "nye"))
  (bind _returnvalue_6 (select `int` (`KismetMathLibrary.RandomIntegerInRangeFromStream` 0 26 (`KismetMathLibrary.MakeRandomStream` (+ (* _returnvalue 3) 16 _attemptnum))) :`0` "ia" :`1` "i" :`2` "en" :`3` "us" :`4` "ius" :`5` "tac" :`6` "lin" :`7` "ria" :`8` "io" :`9` "'ke" :`10` "'ka" :`11` "sa" :`12` "ya" :`13` "wat" :`14` "'tel" :`15` "laa" :`16` "op" :`17` "we" :`18` "uo" :`19` "iao" :`20` "iat" :`21` "ae" :`22` "uus" :`23` "en" :`24` "ga" :`25` "ya" :`26` "no"))
  (bind _returnvalue_7 (select `bool` (`KismetStringLibrary.EqualEqual_StrStr` _returnvalue_3 "Lava") :`true` 1.0 :!type "Float (single-precision)"))
  (bind _returnvalue_8 (select `bool` (`KismetStringLibrary.EqualEqual_StrStr` _returnvalue_3 "Ice") :`true` 1.0 :!type "Float (single-precision)"))
  (bind _returnvalue_9 (select `int` (`KismetMathLibrary.RandomIntegerInRangeFromStream` 0 3 (`KismetMathLibrary.MakeRandomStream` (+ (* _returnvalue 7) 17 _attemptnum))) :`0` (`KismetStringLibrary.Concat_StrStr` _returnvalue_4 _returnvalue_5 _returnvalue_6) :`1` (`KismetStringLibrary.Concat_StrStr` _returnvalue_4 _returnvalue_5) :`2` (`KismetStringLibrary.Concat_StrStr` _returnvalue_4 _returnvalue_6) :`3` (`KismetStringLibrary.Concat_StrStr` (select `int` _returnvalue_2 :`0` "No" :`1` "Baan" :`2` "Mu" :`3` "Bis" :`4` "Ten" :`5` "Ris" :`6` "Gand" :`7` "Be" :`8` "To" :`9` "Kuu" :`10` "In" :`11` "Ho" :`12` "Yu" :`13` "Wen" :`14` "Ju" :`15` "Ken" :`16` "Go" :`17` "Ta" :`18` "Mar" :`19` "Bo" :`20` "Rad" :`21` "Ven" :`22` "Fre" :`23` "Shi" :`24` "Sen" :`25` "La" :`26` "Wi" :`27` "Bi'" :`28` "Nye") _returnvalue_6)))
  (bind _returnvalue_10 (select `int` (`KismetMathLibrary.RandomIntegerInRangeFromStream` 0 1 (`KismetMathLibrary.MakeRandomStream` (+ _returnvalue 19 _attemptnum))) :`0` _returnvalue_9 :`1` (`KismetStringLibrary.Concat_StrStr` _returnvalue_9 (select `int` (`KismetMathLibrary.RandomIntegerInRangeFromStream` 0 10 (`KismetMathLibrary.MakeRandomStream` (+ _returnvalue 18 _attemptnum))) :`0` "-II" :`1` "-I" :`2` "-III" :`3` "-IV" :`4` "-V" :`5` "-VI" :`6` "-VII" :`7` "-VIII" :`8` "-IX" :`9` "-X" :`10` "-XI"))))
  ;[1 1 1] Name Check
  (set `self.PlanetNameMatch` false)
  (bind _output_get (set `self.TempName` _returnvalue_10))
  (bind _planetnames (`/Game/Blueprints/BP_SpaceGameInstance.PlanetNames` (stale `self.ReceiveBeginPlay` _asbp_space_game_instance)))
  (for _array_element _planetnames
    (if (`KismetStringLibrary.EqualEqual_StrStr` _output_get _array_element)
      (set `self.PlanetNameMatch` true)
      (break)))
  (if (`self.PlanetNameMatch`)
    (if (not (== (`self.AttemptNum`) 3))
      (set `self.AttemptNum` (+ (`self.AttemptNum`) 1))
      (`self.AttemptPlanetBuild`))
    (else
      (`KismetArrayLibrary.Array_Add` _planetnames _output_get)
      ;[1 1 1] Planet Surface Generator
      (`self.Apply Planet Attributes` _returnvalue_3 (`KismetMathLibrary.RandomFloatInRangeFromStream` 0.7 3.0 (`KismetMathLibrary.MakeRandomStream` (+ _returnvalue 11))) (`self.PrimaryColor`) (`self.SecondaryColor`) (`self.ThirdColor`) (stale `self.ReceiveBeginPlay` _output_get) (`KismetMathLibrary.RandomUnitVectorFromStream` (`KismetMathLibrary.MakeRandomStream` (+ _returnvalue 5))) (`KismetMathLibrary.RandomUnitVectorFromStream` (`KismetMathLibrary.MakeRandomStream` (+ _returnvalue 6))) (`KismetStringLibrary.Conv_StringToName` _returnvalue_10))
      (`MeshComponent.SetScalarParameterValueOnMaterials` _planetmesh "Ice?" _returnvalue_8)
      (`MeshComponent.SetScalarParameterValueOnMaterials` _planetmesh "Lava?" _returnvalue_7)
      (`MaterialInstanceDynamic.SetScalarParameterValue` _planetmapui "Ice?" _returnvalue_8)
      (`MaterialInstanceDynamic.SetScalarParameterValue` _planetmapui "Lava?" (* _returnvalue_7 0.5))
      (`self.LandLayout`)
      (bind _returnvalue_11 (`CanvasRenderTarget2D.CreateCanvasRenderTarget2D` "/Game/Blueprints/BP_PlanetCanvas.BP_PlanetCanvas_C" 18 9))
      (bind _output_get_2 (set `self.MapCanvasRender` _returnvalue_11))
      (add `CanvasRenderTarget2D.OnCanvasRenderTargetUpdate` _output_get_2 (delegate `DrawMap`))
      (`CanvasRenderTarget2D.UpdateResource` _output_get_2))))

(event `self.ReceiveTick`
  (params (DeltaSeconds :type "Float (single-precision)"))
  ;[1 0.9185 0.322] Planet Rotation
  (`|ExecutionSequence`
    (:`then_0`
      (`SceneComponent.K2_AddLocalRotation` (`self.PlanetMesh`) (struct :`Yaw` 0.1) false false))
    (:`then_1`
      (bind _output_get (set `self.OrbitVector` (`KismetMathLibrary.GreaterGreater_VectorRotator` (`self.OrbitVector`) (`KismetMathLibrary.MakeRotator` 0.0 0.0 (`KismetMathLibrary.RandomFloatInRangeFromStream` 0.001 0.03 (`KismetMathLibrary.MakeRandomStream` (+ (`KismetMathLibrary.FTrunc` (+ (.x (`self.PlanetPos`)) (.y (`self.PlanetPos`)) (.z (`self.PlanetPos`)))) (`self.gSeed`) (`self.PlanetNum`))))))))
      (`self.K2_SetActorLocation` (+ _output_get (`self.K2_GetActorLocation` (`self.GetOwner`)))))))

(event `self.ReceiveBeginPlay`
  (bind _returnvalue (+ (`KismetMathLibrary.FTrunc` (+ (.x (`self.PlanetPos`)) (.y (`self.PlanetPos`)) (.z (`self.PlanetPos`)))) (`self.gSeed`) (`self.PlanetNum`)))
  (bind _returnvalue_2 (`KismetMathLibrary.FClamp` (- 1.6 (+ (+ (`KismetMathLibrary.RandomFloatInRangeFromStream` 0.0 1.0 (`KismetMathLibrary.MakeRandomStream` (+ _returnvalue 7))) (`KismetMathLibrary.RandomFloatInRangeFromStream` 0.0 1.0 (`KismetMathLibrary.MakeRandomStream` (+ _returnvalue 8)))) (`KismetMathLibrary.RandomFloatInRangeFromStream` 0.0 1.0 (`KismetMathLibrary.MakeRandomStream` (+ _returnvalue 9))))) 0.0 0.4))
  ;[1 0.3088 0.6704] Planet Color Generator
  (bind _asbp_space_game_instance (cast `/Game/Blueprints/BP_SpaceGameInstance` (`GameplayStatics.GetGameInstance`)))
  (set `self.PrimaryColor` (`KismetMathLibrary.MakeVector` (`KismetMathLibrary.Abs` (.x (`KismetMathLibrary.RandomUnitVectorFromStream` (`KismetMathLibrary.MakeRandomStream` _returnvalue)))) (`KismetMathLibrary.Abs` (.y (`KismetMathLibrary.RandomUnitVectorFromStream` (`KismetMathLibrary.MakeRandomStream` _returnvalue)))) (`KismetMathLibrary.Abs` (.z (`KismetMathLibrary.RandomUnitVectorFromStream` (`KismetMathLibrary.MakeRandomStream` _returnvalue))))))
  (set `self.SecondaryColor` (+ (`self.PrimaryColor`) (`KismetMathLibrary.MakeVector` (`KismetMathLibrary.FClamp` (.x (`KismetMathLibrary.RandomUnitVectorFromStream` (`KismetMathLibrary.MakeRandomStream` (+ _returnvalue 1)))) -0.5 0.5) (`KismetMathLibrary.FClamp` (.y (`KismetMathLibrary.RandomUnitVectorFromStream` (`KismetMathLibrary.MakeRandomStream` (+ _returnvalue 1)))) -0.5 0.5) (`KismetMathLibrary.FClamp` (.z (`KismetMathLibrary.RandomUnitVectorFromStream` (`KismetMathLibrary.MakeRandomStream` (+ _returnvalue 1)))) -0.5 0.5))))
  (set `self.ThirdColor` (`KismetMathLibrary.ClampVectorSize` (`KismetMathLibrary.MakeVector` (`KismetMathLibrary.RandomFloatInRangeFromStream` 0.0 1.0 (`KismetMathLibrary.MakeRandomStream` (+ _returnvalue 2))) (`KismetMathLibrary.RandomFloatInRangeFromStream` 0.0 1.0 (`KismetMathLibrary.MakeRandomStream` (+ _returnvalue 3))) (`KismetMathLibrary.RandomFloatInRangeFromStream` 0.0 1.0 (`KismetMathLibrary.MakeRandomStream` (+ _returnvalue 4)))) 0.5 1.0))
  (bind _output_get (set `self.WaterCover` (select `bool` (`KismetStringLibrary.EqualEqual_StrStr` (select `int` (`KismetMathLibrary.RandomIntegerInRangeFromStream` 0 7 (`KismetMathLibrary.MakeRandomStream` (+ _returnvalue 10))) :`0` "Rocky" :`1` "Jungle" :`2` "Ice" :`3` "Lava" :`4` "Swamp" :`5` "Sand" :`6` "Temperate" :`7` "Tropical") "Lava") :`false` _returnvalue_2 :`true` (`KismetMathLibrary.FClamp` _returnvalue_2 0.0 0.1))))
  (`self.AttemptPlanetBuild`))

(event `DrawMap`
  (params (Canvas :type "Canvas Object Reference") (Width :type Integer) (Height :type Integer))
  ;[1 1 1] Planet Surface Generator
  (for (_array_element _array_index) (`self.LandValues`)
    (bind (_x_coord _y_coord) (`self.1Dto2D` (`KismetMathLibrary.Conv_IntToDouble` _array_index) (`self.MapSizeX`)))
    (`Canvas.K2_DrawTexture` Canvas null (`KismetMathLibrary.MakeVector2D` (`KismetMathLibrary.Conv_IntToDouble` _x_coord) (`KismetMathLibrary.Conv_IntToDouble` _y_coord)) (1.0 1.0) (0.0 0.0) (1.0 1.0) (`KismetMathLibrary.Conv_DoubleToLinearColor` _array_element) "BLEND_Opaque" 0.0 (0.5 0.5)))
  (`MaterialInstanceDynamic.SetTextureParameterValue` (`self.PlanetMatInstance`) "Land" (stale `AttemptPlanetBuild` _returnvalue_11))
  (`MaterialInstanceDynamic.SetTextureParameterValue` (`self.PlanetMapUI`) "Land" (stale `AttemptPlanetBuild` _returnvalue_11)))

(fn `1Dto2D`
  (params (`1DArray` :type "Float (double-precision)") (XDim :type "Float (double-precision)"))
  (returns (`X Coord` :type Integer) (`Y Coord` :type Integer))
  (bind _returnvalue (`KismetMathLibrary.FFloor` (/ `1DArray` XDim)))
  (return (`KismetMathLibrary.FFloor` (- `1DArray` (* _returnvalue XDim))) _returnvalue))

(fn `2Dto1D`
  (params (Xcoord :type Integer) (YCoord :type Integer) (XDim :type Integer))
  (returns (ArrayPos :type Integer))
  (return (+ Xcoord (* YCoord XDim))))

(fn `Apply Planet Attributes`
  (params (Type :type String) (Size :type "Float (double-precision)" :default 0.0) (PrimaryColor :type "Vector Structure") (SecondaryColor :type "Vector Structure") (ThirdColor :type "Vector Structure") (WaterCover :type "Float (double-precision)") (LandSeed1 :type "Vector Structure") (LandSeed2 :type "Vector Structure") (PlanetName :type Name))
  (`|ExecutionSequence`
    (:`then_0`
      (bind _returnvalue (`PrimitiveComponent.CreateDynamicMaterialInstance` (`self.PlanetMesh`) 0 "/Game/Materials/M_PlanetDepth.M_PlanetDepth"))
      (set `self.PlanetMatInstance` _returnvalue)
      (bind _returnvalue_2 (`PrimitiveComponent.CreateDynamicMaterialInstance` (`self.AtmosMesh`) 0 "/Game/Materials/M_Atmosphere.M_Atmosphere"))
      (set `self.AtmosMat` _returnvalue_2)
      (bind _returnvalue_3 (`KismetMaterialLibrary.CreateDynamicMaterialInstance` "/Game/Materials/M_PlanetUI.M_PlanetUI"))
      (set `self.PlanetMapUI` _returnvalue_3))
    (:`then_1`
      (`SceneComponent.SetRelativeScale3D` (`self.PlanetMesh`) (`KismetMathLibrary.Conv_DoubleToVector` Size)))
    (:`then_2`
      (`self.SetPlanetMatAttr` (`self.PlanetMatInstance`) PrimaryColor SecondaryColor ThirdColor WaterCover LandSeed1 LandSeed2))
    (:`then_3`
      (`self.SetPlanetMatAttr` (`self.PlanetMapUI`) PrimaryColor SecondaryColor ThirdColor WaterCover LandSeed1 LandSeed2))
    (:`then_4`
      (`MaterialInstanceDynamic.SetVectorParameterValue` (`self.AtmosMat`) "ThirdColor" (`KismetMathLibrary.Conv_VectorToLinearColor` ThirdColor)))
    (:`then_5`
      (set `self.Type` Type)
      (set `self.PlanetName` PlanetName))))

(fn `LandLayout`
  (bind _gseed (`self.gSeed`))
  (bind _landvalues (`self.LandValues`))
  (bind _returnvalue (`KismetMathLibrary.FTrunc` (* (`self.MapSizeX`) (`self.MapSizeY`))))
  (`|ExecutionSequence`
    (:`then_0`
      (for _index (range 1 (+ _returnvalue 1))
        ;[0.4331 1 0.3352] Generate Random Land Values
        (if (< (`KismetArrayLibrary.Array_Length` _landvalues) _returnvalue)
          (`KismetArrayLibrary.Array_Add` _landvalues (`KismetMathLibrary.RandomFloatInRangeFromStream` 0.0 1.0 (`KismetMathLibrary.MakeRandomStream` (* (`KismetMathLibrary.FTrunc` (* (+ (- _gseed (* (/ _gseed 10) 10)) _index) (+ (.x (`self.PlanetPos`)) (* (.y (`self.PlanetPos`)) 100.0) (* (.z (`self.PlanetPos`)) 10000.0)))) _index)))))))))

(fn `UserConstructionScript`)