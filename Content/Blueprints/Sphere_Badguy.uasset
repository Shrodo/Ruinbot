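; Sphere enemy that chases any SpaceCharacter inside its detection sphere, otherwise moving to its spawn or last-seen target location.
; Damage lowers Health, shown by a debug-drawn ring; a hit arriving at zero or below starts a one-second death timer before destruction.
; Tick turns timer progress, including an empty-event timer for hit flashes, into dynamic material parameters.
; Twin-stick FireShot logic exists but is never triggered.
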(event `nothing`)

(event `self.ReceiveAnyDamage`
  (params (Damage :type "Float (single-precision)") (DamageType :type "DamageType Object Reference") (InstigatedBy :type "Controller Object Reference") (DamageCauser :type "Actor Object Reference"))
  (bind _health (`self.Health`))
  (if (<= _health 0.0)
    (if (not (`self.Dead`))
      (set `self.Dead` true)
      (`self.DeathTime`))
    (else
      (set `self.Health` (- _health Damage))
      (bind _returnvalue (`KismetSystemLibrary.K2_SetTimerDelegate` (delegate `nothing`) 0.2)))))

(event `self.ReceiveBeginPlay`
  (set `self.HuntLoc` (`SceneComponent.K2_GetComponentLocation` (`self.Mesh`)))
  (bind _returnvalue (`PrimitiveComponent.CreateDynamicMaterialInstance` (`self.StaticMesh`) 0 "/Game/Materials/M_SphereBadguy.M_SphereBadguy" "None"))
  (`PrimitiveComponent.SetMaterial` (`self.StaticMesh1`) 0 _returnvalue))

(event `self.ReceiveTick`
  (params (DeltaSeconds :type "Float (single-precision)"))
  (bind _returnvalue (`self.GetController`))
  (bind _health (`self.Health`))
  (bind _overlappingactors (`PrimitiveComponent.GetOverlappingActors` (`self.Sphere`) null "/Game/Blueprints/SpaceCharacter.SpaceCharacter_C"))
  (`|ExecutionSequence`
    (:`then_0`
      (`KismetSystemLibrary.DrawDebugCircle` (+ (`SceneComponent.K2_GetComponentLocation` (`self.CapsuleComponent`)) (0.0 0.0 80.0)) _health 5 (`KismetMathLibrary.LinearColorLerp` (struct :`R` 1.0 :`A` 1.0) (struct :`G` 1.0 :`A` 1.0) (/ _health 100.0)) 0.1 (- 5.0 (/ _health 50.0)) (0.0 1.0 0.0) (1.0 0.0 0.0)))
    (:`then_1`
      (if (> (`KismetArrayLibrary.Array_Length` _overlappingactors) 0)
        (for _array_element _overlappingactors
          (`NavigationSystemV1.SimpleMoveToActor` _returnvalue _array_element)
          (set `self.HuntLoc` (`self.K2_GetActorLocation` _array_element)))
        (else
          (`NavigationSystemV1.SimpleMoveToLocation` _returnvalue (`self.HuntLoc`)))))
    (:`then_2`
      (bind _output_get (set `self.DeathAnim` (- 5.0 (* (`KismetSystemLibrary.K2_GetTimerElapsedTimeHandle` (stale `DeathTime` _returnvalue)) 5.0))))
      (`MaterialInstanceDynamic.SetScalarParameterValue` (stale `self.ReceiveBeginPlay` _returnvalue) "DeathTimer" _output_get)
      (`MaterialInstanceDynamic.SetScalarParameterValue` (stale `self.ReceiveBeginPlay` _returnvalue) "HealthColor" (`KismetMathLibrary.FClamp` (* (`KismetSystemLibrary.K2_GetTimerRemainingTimeHandle` (stale `self.ReceiveAnyDamage` _returnvalue)) 10.0) 0.0 2.0)))))

(event `DeathTime`
  (bind _returnvalue (`KismetSystemLibrary.K2_SetTimerDelegate` (delegate `DeathFin`) 1.0)))

(event `DeathFin`
  (`/Engine/EditorBlueprintResources/StandardMacros.IsValid` self
    (:`Is Valid`
      (`self.K2_DestroyActor`))))

(fn `Fire Shot`
  (params (Direction :type "Vector Structure"))
  (bind _returnvalue (`KismetMathLibrary.Conv_VectorToRotator` (0.0 0.0 0.0)))
  (bind _returnvalue_2 (+ (`self.K2_GetActorLocation`) (`KismetMathLibrary.GreaterGreater_VectorRotator` (`self.GunOffset`) _returnvalue)))
  (if (`self.CanFire`)
    (if (> (`KismetMathLibrary.VSize` Direction) 0.0)
      (`|SpawnActorFromClass` "/Game/Blueprints/TwinStickProjectile.TwinStickProjectile_C" (`KismetMathLibrary.MakeTransform` _returnvalue_2 _returnvalue) "AlwaysSpawn" "OverrideRootScale" null null)
      (`GameplayStatics.PlaySoundAtLocation` (`self.FireSound`) _returnvalue_2 (struct) 1.0 1.0 0.0 null null null)
      (set `self.CanFire` false)
      (`KismetSystemLibrary.K2_SetTimer` null "Shot Timer Expired" (`self.FireRate`)))))

(fn `Shot Timer Expired`
  (set `self.CanFire` true))

(fn `UserConstructionScript`)