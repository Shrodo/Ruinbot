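; BP_DialogueSystem is an actor that runs a branching NPC conversation through an on-screen dialogue widget.
; On BeginPlay it creates W_DialogueScreen and loads the first node of its DialogueTest conversation data.
; LoadDialogue shows the NPC name and reply, then rebuilds choice widgets carrying link and exit data, focusing the first for input.
; An exit request hides the screen, notifies BP_SpacePirateChar and destroys the actor.
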(event `self.ReceiveBeginPlay`
  (bind _returnvalue (`|CreateWidget` "/Game/Spirate/Blueprints/Dialogue/W_DialogueScreen.W_DialogueScreen_C"))
  (bind _output_get (set `self.DialogueWidget` _returnvalue))
  (`UserWidget.AddToViewport` _output_get 0)
  (`self.StartConversation`))

(fn `Load Dialogue`
  (params (`Locate Node` :type Integer) (`Exit Convo` :type Boolean))
  (bind _dialoguewidget (`self.DialogueWidget`))
  (bind (_npc_owner _conversation) (break `/Game/Spirate/Blueprints/Dialogue/ST_DialogueTree` (`self.DialogueTest`)))
  (bind (_npc_reply _pc_choices) (break `/Game/Spirate/Blueprints/Dialogue/ST_NPC_Reply` (`|GetArrayItem` _conversation `Locate Node`)))
  ;[1 1 1] If close is set to true, hide the dialogue screen
  (if `Exit Convo`
    (`Widget.SetVisibility` (`self.DialogueWidget`) "Hidden")
    (bind _asbp_space_pirate_char (cast `/Game/Spirate/Characters/BP_SpacePirateChar` (`GameplayStatics.GetPlayerCharacter` 0)))
    (`/Game/Spirate/Characters/BP_SpacePirateChar.ExitConvo` _asbp_space_pirate_char)
    (`/Engine/EditorBlueprintResources/StandardMacros.IsValid` self
      (:`Is Valid`
        (`self.K2_DestroyActor`)))
    (else
      ;[1 1 1] Remove options from previous screen
      (`PanelWidget.ClearChildren` (`/Game/Spirate/Blueprints/Dialogue/W_DialogueScreen.ChoicesVertBox` _dialoguewidget))
      (`TextBlock.SetText` (`/Game/Spirate/Blueprints/Dialogue/W_DialogueScreen.NPCResponseText` _dialoguewidget) _npc_reply)
      (`TextBlock.SetText` (`/Game/Spirate/Blueprints/Dialogue/W_DialogueScreen.NPCName` _dialoguewidget) (`KismetTextLibrary.Conv_NameToText` _npc_owner))
      (for (_array_element _array_index) _pc_choices
        (bind _returnvalue (`|CreateWidget` "/Game/Spirate/Blueprints/Dialogue/W_Choices.W_Choices_C"))
        (`VerticalBox.AddChildToVerticalBox` (`/Game/Spirate/Blueprints/Dialogue/W_DialogueScreen.ChoicesVertBox` (`self.DialogueWidget`)) _returnvalue)
        (bind (_reply _linktonode _exitconversation) (break `/Game/Spirate/Blueprints/Dialogue/ST_PC_Choices` _array_element))
        (`TextBlock.SetText` (`/Game/Spirate/Blueprints/Dialogue/W_Choices.ChoiceText` _returnvalue) _reply)
        (set `/Game/Spirate/Blueprints/Dialogue/W_Choices.Link to Node` _linktonode _returnvalue)
        (set `/Game/Spirate/Blueprints/Dialogue/W_Choices.Exit Convo` _exitconversation _returnvalue)
        (if (== _array_index 0)
          (`Widget.SetUserFocus` (`/Game/Spirate/Blueprints/Dialogue/W_Choices.ChoiceButton` _returnvalue) (`GameplayStatics.GetPlayerController` 0)))))))

(fn `StartConversation`
  (`self.Load Dialogue` 0))

(fn `UserConstructionScript`)