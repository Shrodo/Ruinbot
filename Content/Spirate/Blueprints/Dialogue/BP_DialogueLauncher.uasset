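; BP_DialogueLauncher is a proximity trigger that shows an interaction prompt to the space pirate character.
; When the character enters its sphere, it stores the character and calls XPrompt with configurable text, button and key, naming itself as instigator.
; When that character leaves, it stops the prompt only if this launcher is still the active prompt actor.
; The file itself contains no dialogue logic.
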(event `self.Sphere.OnComponentBeginOverlap`
  (params (OverlappedComponent :type "PrimitiveComponent Object Reference") (OtherActor :type "Actor Object Reference") (OtherComp :type "PrimitiveComponent Object Reference") (OtherBodyIndex :type Integer) (bFromSweep :type Boolean) (SweepResult :type "HitResult Structure (by ref)"))
  (bind _asbp_space_pirate_char (cast `/Game/Spirate/Characters/BP_SpacePirateChar` OtherActor))
  (bind _output_get (set `self.Character` _asbp_space_pirate_char))
  (`/Game/Spirate/Characters/BP_SpacePirateChar.XPrompt` _output_get (`self.DefaultPrompt?`) (`self.PromptText`) (`self.ButtonID`) (`self.Key`) self))

(event `self.Sphere.OnComponentEndOverlap`
  (params (OverlappedComponent :type "PrimitiveComponent Object Reference") (OtherActor :type "Actor Object Reference") (OtherComp :type "PrimitiveComponent Object Reference") (OtherBodyIndex :type Integer))
  (bind _character (`self.Character`))
  (bind _promptactor (`/Game/Spirate/Characters/BP_SpacePirateChar.PromptActor` _character))
  (`/Engine/EditorBlueprintResources/StandardMacros.IsValid` _character
    (:`Is Valid`
      (if (== OtherActor _character)
        (`/Engine/EditorBlueprintResources/StandardMacros.IsValid` _promptactor
          (:`Is Valid`
            (if (== _promptactor self)
              (`/Game/Spirate/Characters/BP_SpacePirateChar.StopXPrompt` _character))))))))

(fn `UserConstructionScript`)