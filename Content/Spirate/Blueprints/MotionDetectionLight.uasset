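; MotionDetectionLight is a spot light actor that switches on when a Pawn overlaps it and off when a Pawn leaves.
; Actor begin and end overlap events filter for Pawn subclasses, then set the SpotLight intensity to full brightness or zero.
; End overlap does not count remaining occupants, so any departing Pawn turns the light off.
; The construction script applies the LightColor variable to the SpotLight.
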(event `self.ReceiveActorBeginOverlap`
  (params (OtherActor :type "Actor Object Reference"))
  (if (`KismetMathLibrary.ClassIsChildOf` (`GameplayStatics.GetObjectClass` OtherActor) "/Script/Engine.Pawn")
    (`LightComponent.SetIntensity` (`self.SpotLight`) 100000.0)))

(event `self.ReceiveActorEndOverlap`
  (params (OtherActor :type "Actor Object Reference"))
  (if (`KismetMathLibrary.ClassIsChildOf` (`GameplayStatics.GetObjectClass` OtherActor) "/Script/Engine.Pawn")
    (`LightComponent.SetIntensity` (`self.SpotLight`) 0.0)))

(fn `UserConstructionScript`
  (`LightComponent.SetLightColor` (`self.SpotLight`) (`self.LightColor`) true))