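; Galaxy actor that procedurally lays out star systems as static meshes inside a circular area, built entirely in the construction script.
; It walks a grid via index-to-coordinate helpers, centers it on the actor and keeps only cells within Radius.
; Each kept cell gets a flattened random offset from a GalaxySeed-and-index stream, making layouts repeatable.
; Grid coordinates and jittered positions are stored in SystemLocalCoords and SystemLoc.
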(fn `1DArrayTo2DCoords`
  (params (Index :type Integer))
  (returns (CoordX :type Integer) (CoordY :type Integer))
  (bind _gridsizex (`self.GridSizeX`))
  (bind _returnvalue (`KismetMathLibrary.FFloor` (/ (`KismetMathLibrary.Conv_IntToDouble` Index) (`KismetMathLibrary.Conv_IntToDouble` _gridsizex))))
  (return _returnvalue (- Index (* _gridsizex _returnvalue))))

(fn `2DCoordsTo1DArray`
  (params (CoordX :type Integer) (CoordY :type Integer))
  (returns (Index :type Integer))
  (return (+ CoordY (* CoordX (`self.GridSizeX`)))))

(fn `UserConstructionScript`
  (bind _gridsizex (`self.GridSizeX`))
  (bind _gridsizey (`self.GridSizeY`))
  (bind _systemlocalcoords (`self.SystemLocalCoords`))
  (bind _returnvalue (* (`self.Radius`) 2.0))
  (bind _returnvalue_2 (* (`self.GridSizeX`) (`self.GridSizeY`)))
  (bind _returnvalue_3 (/ _returnvalue (`KismetMathLibrary.Conv_IntToDouble` _gridsizex)))
  (bind _returnvalue_4 (/ _returnvalue (`KismetMathLibrary.Conv_IntToDouble` _gridsizey)))
  (`KismetArrayLibrary.Array_Resize` _systemlocalcoords _returnvalue_2)
  (`KismetArrayLibrary.Array_Resize` (`self.SystemLoc`) _returnvalue_2)
  (for (_ _array_index) _systemlocalcoords
    (bind (_coordx _coordy) (`self.1DArrayTo2DCoords` _array_index))
    (bind _returnvalue_5 (* _coordx _returnvalue_4))
    (bind _returnvalue_6 (* _coordy _returnvalue_3))
    (`KismetArrayLibrary.Array_Set` _systemlocalcoords _array_index (`KismetMathLibrary.MakeVector2D` _returnvalue_5 _returnvalue_6))
    (bind _returnvalue_7 (`KismetMathLibrary.MakeVector` (+ _returnvalue_5 (* (`KismetMathLibrary.Conv_IntToDouble` (- _gridsizey 1)) -0.5 _returnvalue_4)) (+ _returnvalue_6 (* (`KismetMathLibrary.Conv_IntToDouble` (- _gridsizex 1)) -0.5 _returnvalue_3))))
    (if (< (`KismetMathLibrary.VSize` _returnvalue_7) (`self.Radius`))
      (bind _returnvalue_8 (+ _returnvalue_7 (* (* (`KismetMathLibrary.RandomUnitVectorFromStream` (`KismetMathLibrary.MakeRandomStream` (+ (* _array_index 1325) (`self.GalaxySeed`)))) (`self.ItemOffsetRand`)) (1.0 1.0 0.0))))
      (`KismetArrayLibrary.Array_Set` (`self.SystemLoc`) _array_index _returnvalue_8)
      (`AddComponent|NODE_AddStaticMeshComponent-0` :`RelativeTransform` (`KismetMathLibrary.MakeTransform` _returnvalue_8 (struct) (`KismetMathLibrary.Conv_DoubleToVector` (`self.ItemScale`)))))))